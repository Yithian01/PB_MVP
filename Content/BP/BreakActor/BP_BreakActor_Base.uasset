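; Base breakable world item that can be grabbed, thrown and destroyed by point damage.
; BPCBreakObject checks hits with a DT_BreakType damage type; on success the game mode destroys the item and updates the break score.
; Grabbing disables physics and pawn collision; release simulates the Body, flags it thrown and starts a short timer.
; The root is parked high above while thrown, then realigned and reattached to the Body when it sleeps.
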(event OnComponentSleep(Body)
  (params (SleepingComponent :type Primitive%20Component%20Object%20Reference) (BoneName :type Name :default "None"))
  ;[0.15 0.15 0.15 0.5] On Sleep
  (Variables|Default|SetbIsThrow false)
  (Collision|SetCollisionResponsetoChannel (Variables|Default|GetBody) "ECC_Pawn" "ECR_Block")
  (Transformation|SetRelativeTransform (Variables|Default|GetDefaultSceneRoot) (Transformation|GetWorldTransform (Variables|Default|GetBody)) false false)
  (Transformation|AttachComponentToComponent (Variables|Default|GetBody) (Variables|Default|GetDefaultSceneRoot) "None" "KeepWorld" "KeepWorld" "KeepWorld" false))

(event Custom|OnReleaseGrabCollision
  ;[0.15 0.15 0.15 0.5] PostReleaseGrab
  (Collision|SetCollisionResponsetoChannel (Variables|Default|GetBody) "ECC_Pawn" "ECR_Block"))

(event EventBeginPlay
  (bind _asbp_game_mode (Utilities|Casting|CastToBP_GameMode (Game|GetGameMode)))
  (Variables|Ref|SetGameModeRef _asbp_game_mode))

(event Game|Damage|EventPointDamage
  (params (Damage :type Float%20%28single-precision%29) (DamageType :type Damage%20Type%20Object%20Reference) (HitLocation :type Vector :default "0, 0, 0") (HitNormal :type Vector :default "0, 0, 0") (HitComponent :type Primitive%20Component%20Object%20Reference) (BoneName :type Name :default "None") (ShotFromDirection :type Vector :default "0, 0, 0") (InstigatedBy :type Controller%20Object%20Reference) (DamageCauser :type Actor%20Object%20Reference) (HitInfo :type Hit%20Result%20Structure%20%28by%20ref%29))
  (bind (_bblockinghit _binitialoverlap _time _distance _location _impactpoint _normal _impactnormal) (Collision|BreakHitResult HitInfo))
  (bind _gamemoderef (Variables|Ref|GetGameModeRef))
  ;[0.15 0.15 0.15 0.5] ApplyDamage
  (bind _asdt_break_type (Utilities|Casting|CastToDT_BreakType DamageType))
  (bind _bisbreak (Default|CheckHit (Variables|Default|GetBPC_BreakObject) (Variables|/Game/BP/Datas/DamageType/DT_BreakType.DT_BreakType_C|GetDamageType _asdt_break_type) (Transformation|GetActorTransform) _impactpoint (* Damage _impactnormal)))
  (if _bisbreak
    (Default|DestroyWorldItem _gamemoderef self)
    (Default|UpdateBreakScore _gamemoderef)))

(fn ConstructionScript)

(fn InitializeWorldItemBaseData
  (params (ItemType :type E_ItemType%20Enum :default "NewEnumerator0") (ItemName :type Text) (UIPrefix :type E_UIPrefix%20Enum :default "NewEnumerator0") (StaticMesh :type Static%20Mesh%20Object%20Reference) (Icon :type Texture%202D%20Object%20Reference) (OutlineAble :type Boolean))
  (|CallParentFunction ItemType ItemName UIPrefix StaticMesh Icon OutlineAble))

(fn InitializeSpawnData
  (params (ID :type Name :default "None") (SN :type String))
  (|CallParentFunction ID SN))

(fn SetOutlineAble
  (params (Value :type Boolean))
  (|CallParentFunction Value))

(fn OnGrabbed
  (Physics|SetSimulatePhysics (Variables|Default|GetBody) false)
  (Transformation|SetRelativeTransform (Variables|Default|GetDefaultSceneRoot) (Transformation|GetWorldTransform (Variables|Default|GetBody)) false false)
  (Transformation|AttachComponentToComponent (Variables|Default|GetBody) (Variables|Default|GetDefaultSceneRoot) "None" "KeepWorld" "KeepWorld" "KeepWorld" false)
  (Collision|SetCollisionResponsetoChannel (Variables|Default|GetBody) "ECC_Pawn" "ECR_Ignore"))

(fn OnReleaseGrab
  (Collision|SetCollisionEnabled (Variables|Default|GetBody) "QueryAndPhysics")
  (Physics|SetSimulatePhysics (Variables|Default|GetBody) true)
  (Transformation|SetWorldLocation (Variables|Default|GetDefaultSceneRoot) "0.000000,0.000000,50000.000000" false false)
  (Variables|Default|SetbIsThrow true)
  (Utilities|Time|SetTimerbyEvent (EventDispatchers|CreateEvent :!event Custom|OnReleaseGrabCollision) 0.1))

(fn IsThrow
  (return (Variables|Default|GetbIsThrow)))

(fn GetArmorType
  (return (Variables|/Game/BP/Components/BreakActorComponent/BPC_BreakObject.BPC_BreakObject_C|GetArmorType (Variables|Default|GetBPC_BreakObject))))