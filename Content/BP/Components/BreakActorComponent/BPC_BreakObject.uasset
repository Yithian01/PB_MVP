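; Actor component that makes an object breakable, swapping in a Geometry Collection after enough matching hits.
; CheckHit ignores hits whose damage type differs from ArmorType, otherwise counts down CurrentHitCounter and returns true only on the breaking hit.
; That hit spawns a GeometryCollectionActor at the supplied transform, assigns the ConvertGC rest collection, applies the impact impulse, then sets collision to query-only.
; The component does not remove the original object itself.
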(event EventBeginPlay)

(fn CheckHit
  (params (DamageType :type E_DamageType%20Enum :default "NewEnumerator0") (ActorTransfrom :type Transform) (ImpactPoint :type Vector) (impactForce :type Vector))
  (if (Utilities|Enum|Equal(Enum) DamageType (Variables|Default|GetArmorType))
    (if (<= (- (Variables|Default|GetCurrentHitCounter) 1) 0)
      (CallFunction|SpawnGCObject ActorTransfrom ImpactPoint impactForce)
      (return true)
      (else
        (Variables|Default|SetCurrentHitCounter (- (Variables|Default|GetCurrentHitCounter) 1))
        (return false)))
    (else
      (return false))))

(fn SpawnGCObject
  (params (SpawnTransfrom :type Transform) (ImpactPoint :type Vector) (ImpactForce :type Vector))
  (bind _returnvalue (Game|SpawnActorfromClass "/Script/GeometryCollectionEngine.GeometryCollectionActor" SpawnTransfrom "AlwaysSpawn" "MultiplyWithRoot" 0 0))
  (bind _output_get (LocalVariables|SetSpawnActor (Variables|/Script/GeometryCollectionEngine.GeometryCollectionActor|GetGeometryCollectionComponent _returnvalue)))
  (Class|GeometryCollectionComponent|SetRestCollection _output_get (Variables|Default|GetConvert_GC) true)
  (Physics|AddImpulseatLocation (LocalVariables|GetSpawnActor) ImpactForce ImpactPoint "None")
  (Collision|SetCollisionEnabled (LocalVariables|GetSpawnActor) "QueryOnly"))