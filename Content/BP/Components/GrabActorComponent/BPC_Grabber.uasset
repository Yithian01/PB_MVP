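; BPC_Grabber is a component that tracks a single grabbed item for its owner.
; TryGrab stores an item only when nothing valid is held, and ReleaseGrab clears the slot and returns what it held.
; IsGrab reports whether an item is held, and GetGrabItemArmorType forwards its armor type or falls back to a default enum value.
; It only manages the reference, with no attachment or physics logic.
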(event EventBeginPlay)

(fn ReleaseGrab
  (Utilities|IsValid (Variables|Default|GetCurrentGrabItem)
    (:Is%20Valid
      (LocalVariables|SetReturnGrabItem (Variables|Default|GetCurrentGrabItem))
      (Variables|Default|SetCurrentGrabItem 0)
      (return (LocalVariables|GetReturnGrabItem)))))

(fn TryGrab
  (params (GrabItem :type BP%20Break%20Actor%20Base%20Object%20Reference))
  (Utilities|IsValid (Variables|Default|GetCurrentGrabItem)
    (:Is%20Valid
      (return false))
    (:Is%20Not%20Valid
      (Variables|Default|SetCurrentGrabItem GrabItem)
      (return true))))

(fn IsGrab
  (Utilities|IsValid (Variables|Default|GetCurrentGrabItem)
    (:Is%20Valid
      (return true))
    (:Is%20Not%20Valid
      (return false))))

(fn GetGrabItemArmorType
  (Utilities|IsValid (Variables|Default|GetCurrentGrabItem)
    (:Is%20Valid
      (return (Default|GetArmorType (Variables|Default|GetCurrentGrabItem))))
    (:Is%20Not%20Valid
      (return "NewEnumerator0"))))