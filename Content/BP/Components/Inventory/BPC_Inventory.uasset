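; Inventory component that stores items in an array of slots with one selected quick slot.
; AddItem writes a new item struct into the first slot whose ItemId is None, found by PlaceIndex, without merging stacks.
; SelectQuickSlot moves the selection and returns that slot's ItemId, while RemoveItem clears the selected slot.
; Changes are broadcast through OnUpdateItem and OnSelectQuickSlot so listeners can react.
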(event EventBeginPlay)

(fn AddItem
  (params (ItemType :type E_ItemType%20Enum :default "NewEnumerator0") (ItemItd :type Name) (Amount :type Integer) (Icon :type Texture%202D%20Object%20Reference))
  (LocalVariables|SetCurrentItem (Utilities|Struct|MakeST_InventoryItem ItemType ItemItd Amount Icon))
  (LocalVariables|SetCurrentAddIndex (CallFunction|PlaceIndex))
  (if (>= (LocalVariables|GetCurrentAddIndex) 0)
    (Utilities|Array|SetArrayElem (Variables|Default|GetItems) (LocalVariables|GetCurrentAddIndex) (LocalVariables|GetCurrentItem))
    (Default|CallOnUpdateItem (LocalVariables|GetCurrentAddIndex) (LocalVariables|GetCurrentItem))
    (return true)))

(fn SelectQuickSlot
  (params (Index :type Integer))
  (LocalVariables|SetCurrentItemId (.ItemId (Utilities|Struct|BreakST_InventoryItem (Utilities|Array|Get(acopy) (Variables|Default|GetItems) (Variables|Default|GetCurrentSelectIndex)))))
  (if (== Index (Variables|Default|GetCurrentSelectIndex))
    (return (LocalVariables|GetCurrentItemId))
    (else
      (Default|CallOnSelectQuickSlot (Variables|Default|GetCurrentSelectIndex) Index)
      (Variables|Default|SetCurrentSelectIndex Index)
      (LocalVariables|SetCurrentItemId (.ItemId (Utilities|Struct|BreakST_InventoryItem (Utilities|Array|Get(acopy) (Variables|Default|GetItems) (Variables|Default|GetCurrentSelectIndex)))))
      (return (LocalVariables|GetCurrentItemId)))))

(fn PlaceIndex
  (bind (_array_element _array_index) (Utilities|Array|ForEachLoopwithBreak (Variables|Default|GetItems))
    (:LoopBody
      (if (== (.itemid _array_element) "")
        (return _array_index)))
    (:Completed
      (return -1))))

(fn RemoveItem
  (LocalVariables|SetEmptyItem (Utilities|Struct|MakeST_InventoryItem "NewEnumerator1" "None" 0 0))
  (Utilities|Array|SetArrayElem (Variables|Default|GetItems) (Variables|Default|GetCurrentSelectIndex) (LocalVariables|GetEmptyItem))
  (Default|CallOnUpdateItem (Variables|Default|GetCurrentSelectIndex) (LocalVariables|GetEmptyItem)))