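; BPC_StunSystem is a component that tracks a stun health pool and flags its owner as stunned when that pool is depleted.
; It fills HP on BeginPlay, and TakeDamage subtracts damage, clamps at zero, sets the stun flag and returns true on depletion, ignoring hits while stunned.
; Stun clearing and HP recovery are exposed as separate functions, and HP changes broadcast through an update dispatcher call.
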(event EventBeginPlay
  (Variables|Default|SetCurrentHp (Variables|Default|GetMaxHp))
  (Default|CallOnUpdateHp (Variables|Default|GetCurrentHp) (Variables|Default|GetMaxHp))
  (Variables|Default|SetbIsStuning false))

(event EventTick
  (params (DeltaSeconds :type Float%20%28single-precision%29)))

(fn TakeDamage
  (params (AlppyDamage :type Float%20%28double-precision%29))
  (if (not (Variables|Default|GetbIsStuning))
    (Development|PrintString (Utilities|String|ToString(Float) AlppyDamage))
    (if (<= (- (Variables|Default|GetCurrentHp) AlppyDamage) 0.0)
      (Variables|Default|SetCurrentHp 0.0)
      (Default|CallOnUpdateHp (Variables|Default|GetCurrentHp) (Variables|Default|GetMaxHp))
      (Variables|Default|SetbIsStuning true)
      (return true)
      (else
        (Variables|Default|SetCurrentHp (- (Variables|Default|GetCurrentHp) AlppyDamage))
        (Default|CallOnUpdateHp (Variables|Default|GetCurrentHp) (Variables|Default|GetMaxHp))
        (return false)))))

(fn EnableStun
  (params (bIsEnable :type Boolean))
  (Variables|Default|SetbIsStuning bIsEnable))

(fn RecoverHp
  (params (NewHp :type Float%20%28double-precision%29))
  (Variables|Default|SetCurrentHp NewHp)
  (Default|CallOnUpdateHp (Variables|Default|GetCurrentHp) (Variables|Default|GetMaxHp)))

(fn InitializeHp
  (Default|CallOnUpdateHp (Variables|Default|GetCurrentHp) (Variables|Default|GetMaxHp)))