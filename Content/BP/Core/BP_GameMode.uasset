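; Game mode for a timed, scored stage involving weapon items, a delivery zone and breakable objects.
; On BeginPlay it binds to the delivery zone, spawns a world weapon per data table row at random item-group transforms, and starts a looping countdown.
; It also spawns and destroys items for inventory pickup and throwing.
; At time-out, zone score plus break bonus over the goal sets a table-driven rank before results show.
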(event Custom|GameOver
  ;[0.15 0.15 0.15 0.5] 결과창 띄우기
  (Utilities|FlowControl|Delay 1.0)
  (Score|CalculateRank)
  (Default|CallShowGameResult))

(event EventBeginPlay
  (Utilities|FlowControl|Sequence
    (:then_0
      (bind _returnvalue (Actor|GetActorOfClass "/Game/BP/Truck/BP_DeliveryZone.BP_DeliveryZone_C"))
      (bind _output_get (Variables|Score|SetScoreZone _returnvalue))
      (EventDispatchers|BindEventtoOnUpdateScoreZone _output_get (EventDispatchers|CreateEvent :!event UpdateSocre)))
    (:then_1
      (WorldItem|GenerateWorldItemWeapon))
    (:then_2
      (Variables|Time|SetRemainingTime (Variables|Time|GetGameTime))
      (Utilities|Time|SetTimerbyEvent (EventDispatchers|CreateEvent :!event UpdateGameTimer) 1.0 true))))

(event EventTick
  (params (DeltaSeconds :type Float%20%28single-precision%29))
  (Development|PrintString (Utilities|String|ToString(Text) (Utilities|Text|FormatText "TO BP_GameMode 
 
현재 ZoneScore : {0} 
현재 BreakScore : {1}" (Variables|Score|GetZoneScore) (Variables|Score|GetBreakBonusScore))) true true "(R=0.000000,G=0.660000,B=1.000000,A=1.000000)" 0.0))

(fn ConstructionScript)

(fn DestroyWorldItem
  (params (TargetWorldItem :type BP%20World%20Item%20Base%20Object%20Reference))
  (Actor|DestroyActor TargetWorldItem))

(fn GenerateInventoryItemWeapon
  (params (ItemId :type Name))
  (Utilities|FlowControl|Sequence
    (:then_0
      (bind _returnvalue (Game|SpawnActorfromClass "/Game/BP/Items/InventoryItem/BP_InventoryItem_Weapon.BP_InventoryItem_Weapon_C" (Math|Transform|MakeTransform "0, 0, 0") "AdjustIfPossibleButAlwaysSpawn" "MultiplyWithRoot" 0 0))
      (bind _asbp_inventory_item_base (Utilities|Casting|CastToBP_InventoryItem_Base _returnvalue))
      (bind _output_get (LocalVariables|SetSpawnInventoryItem _asbp_inventory_item_base))
      (Utilities|Array|Add (Variables|Item|GetInventoryItemArr) _output_get))
    (:then_1
      (Default|InitializeSpawnData (LocalVariables|GetSpawnInventoryItem) ItemId)
      (return (LocalVariables|GetSpawnInventoryItem)))))

(fn DestroyInventoryItem
  (params (EquippedItem :type BP%20Inventory%20Item%20Base%20Object%20Reference))
  (Actor|DestroyActor EquippedItem))

(fn GenerateInventorytoWorldItem
  (params (GetTransform :type Transform) (Id :type Name) (ThrowImpulse :type Vector))
  (bind _returnvalue (Game|SpawnActorfromClass "/Game/BP/Items/WorldItem/BP_WorldItem_Weapon.BP_WorldItem_Weapon_C" GetTransform "AdjustIfPossibleButAlwaysSpawn" "MultiplyWithRoot" 0 0))
  (bind _asbp_world_item_base (Utilities|Casting|CastToBP_WorldItem_Base _returnvalue))
  (bind _output_get (LocalVariables|SetCurrentItem _asbp_world_item_base))
  (Utilities|Array|Add (Variables|Item|GetWorldItemArr) _output_get)
  (Default|InitializeSpawnData (LocalVariables|GetCurrentItem) Id)
  (Default|OnDropItem (LocalVariables|GetCurrentItem) ThrowImpulse))

(fn GenerateWorldItemWeapon
  (Utilities|FlowControl|Sequence
    (:then_0
      (bind _returnvalue (Utilities|GetDataTableRow "/Game/BP/Datas/Datatable/ItemGenerater/DT_GroupLocation.DT_GroupLocation" "Stage_1")
        (:then
          (bind _returnvalue_2 (Game|SpawnActorfromClass "/Game/BP/Items/ItemGroup/BP_ItemGroup.BP_ItemGroup_C" (Math|Transform|MakeTransform (.location _returnvalue) "0, 0, 0" "1.000000,1.000000,1.000000") "AdjustIfPossibleButAlwaysSpawn" "MultiplyWithRoot" 0 0))
          (LocalVariables|SetCurrentSpawnLocation _returnvalue_2)
          (bind _outrownames (DataTable|GetDataTableRowNames "/Game/BP/Datas/Datatable/Item/DT_WorldItem_WeaponData.DT_WorldItem_WeaponData"))
          (bind _output_get (LocalVariables|SetWeaponItemRowNames _outrownames))
          (bind _returntransform (Default|GetRandomTransforms (LocalVariables|GetCurrentSpawnLocation) (Utilities|Array|Length _output_get)))
          (LocalVariables|SetCurrentSpawnTransform _returntransform))))
    (:then_1
      (Utilities|Array|Clear (Variables|Item|GetWeaponItemArr))
      (for (_array_element _array_index) (LocalVariables|GetWeaponItemRowNames)
        (bind _returnvalue_3 (Game|SpawnActorfromClass "/Game/BP/Items/WorldItem/BP_WorldItem_Weapon.BP_WorldItem_Weapon_C" (Utilities|Array|Get(acopy) (LocalVariables|GetCurrentSpawnTransform) _array_index) "AdjustIfPossibleButAlwaysSpawn" "MultiplyWithRoot" 0 0))
        (bind _asbp_world_item_base (Utilities|Casting|CastToBP_WorldItem_Base _returnvalue_3))
        (Utilities|Array|Add (Variables|Item|GetWorldItemArr) _asbp_world_item_base)
        (Default|InitializeSpawnData _asbp_world_item_base _array_element)))))

(fn UpdateSocre
  (params (NewBreakItem :type BP%20Break%20Actor%20Base%20Object%20Reference))
  (if (Utilities|Set|Contains (Variables|Score|GetBreakItemList) NewBreakItem)
    (Variables|Score|SetZoneScore (- (Variables|Score|GetZoneScore) (Variables|/Game/BP/BreakActor/BP_BreakActor_Base.BP_BreakActor_Base_C|GetBsaeScore NewBreakItem)))
    (Utilities|Set|Remove (Variables|Score|GetBreakItemList) NewBreakItem)
    (else
      (Utilities|Set|Add (Variables|Score|GetBreakItemList) NewBreakItem)
      (bind _valuepin (Utilities|Set|ForEachLoop(Set) (Variables|Score|GetBreakItemList))
        (:then
          (LocalVariables|SetCurrentSocore (+ (LocalVariables|GetCurrentSocore) (Variables|/Game/BP/BreakActor/BP_BreakActor_Base.BP_BreakActor_Base_C|GetBsaeScore _valuepin))))
        (:CompletedPin
          (Variables|Score|SetZoneScore (LocalVariables|GetCurrentSocore)))))))

(fn UpdateGameTimer
  (Math|Float|DecrementFloat (Variables|Time|GetRemainingTime)
    (:%20%20
      (if (>= (Variables|Time|GetRemainingTime) 0.0)
        (Default|CallOnUpdateGameTime (Variables|Time|GetRemainingTime))
        (elif (not (Variables|Time|GetbIsGameEnd))
          (CallFunction|GameOver)
          (Variables|Time|SetbIsGameEnd true))))))

(fn UpdateBreakScore
  (Math|Integer|IncrementInt (Variables|Score|GetBreakObjectAmount)
    (:%20%20
      (Variables|Score|SetBreakBonusScore (+ (Variables|Score|GetBreakBonusScore) (Variables|Score|GetBreakObjectScore))))))

(fn CalculateRank
  (LocalVariables|SetCurrentModifier (/ (Math|Conversions|ToFloat(Integer) (+ (Variables|Score|GetZoneScore) (Variables|Score|GetBreakBonusScore))) (Math|Conversions|ToFloat(Integer) (Variables|Score|GetGoalScore))))
  (bind _outrownames (DataTable|GetDataTableRowNames "/Game/BP/Datas/Datatable/Score/DT_ScoreGrade.DT_ScoreGrade"))
  (bind _array_element (Utilities|Array|ForEachLoopwithBreak _outrownames :!label _label)
    (:LoopBody
      (bind _returnvalue (Utilities|GetDataTableRow "/Game/BP/Datas/Datatable/Score/DT_ScoreGrade.DT_ScoreGrade" _array_element)
        (:then
          (if (>= (LocalVariables|GetCurrentModifier) (.modifier _returnvalue))
            (Variables|Score|SetRank (.rank _returnvalue))
            (goto _label Break)))))))