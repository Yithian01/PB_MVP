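; Game mode for a timed delivery match that tracks zone score and break bonus, then ranks the result against a goal.
; On BeginPlay it binds to the delivery zone, spawns weapon pickups from data tables and starts a countdown pushed to BP_GameState.
; It converts items between pickable and equipped actors using DT_EquipItemData.
; Broken items are replaced by replicated GeometryCollection actors, and game over grades the score via DT_ScoreGrade.
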(event Custom|GameOver
  ;[0.15 0.15 0.15 0.5] 결과창 띄우기
  (Utilities|FlowControl|Delay 1.0)
  (Score|CalculateRank)
  (Default|CallShowGameResult)
  (Utilities|Time|ClearandInvalidateTimerbyHandle (Variables|TimerHandler|GetTH_GameTimer)))

(event EventBeginPlay
  (Utilities|FlowControl|Sequence
    (:then_0
      (Variables|Default|SetbUseSeamlessTravel true))
    (:then_1
      (bind _returnvalue (Actor|GetActorOfClass "/Game/BP/Game/Truck/BP_DeliveryZone.BP_DeliveryZone_C"))
      (bind _output_get (Variables|Score|SetScoreZone _returnvalue))
      (EventDispatchers|BindEventtoOnUpdateScoreZone _output_get (EventDispatchers|CreateEvent :!event UpdateSocre)))
    (:then_2
      (WorldItem|GenerateWorldItemWeapon))
    (:then_3
      (Variables|Time|SetRemainingTime (Variables|Time|GetGameTime))
      (bind _returnvalue_2 (Utilities|Time|SetTimerbyEvent (EventDispatchers|CreateEvent :!event UpdateGameTimer) 1.0 true))
      (bind _structout (Utilities|Struct|SetmembersinTimerHandle _returnvalue_2))
      (Variables|TimerHandler|SetTH_GameTimer _structout))))

(event Custom|S2M_SpawnBreakActor
  (params (InConvertItem :type Geometry%20Collection%20Object%20Reference) (InDestroyItem :type Actor%20Object%20Reference))
  (bind _returnvalue (Game|SpawnActorfromClass "/Script/GeometryCollectionEngine.GeometryCollectionActor" (Transformation|GetActorTransform InDestroyItem) "AlwaysSpawn" "MultiplyWithRoot" 0 0))
  (Networking|SetReplicates _returnvalue true)
  (Class|Actor|SetReplicateMovement _returnvalue true)
  (Class|GeometryCollectionComponent|SetRestCollection (Variables|/Script/GeometryCollectionEngine.GeometryCollectionActor|GetGeometryCollectionComponent _returnvalue) InConvertItem true)
  (Collision|SetCollisionEnabled (Variables|/Script/GeometryCollectionEngine.GeometryCollectionActor|GetGeometryCollectionComponent _returnvalue) "PhysicsOnly")
  (Actor|DestroyActor InDestroyItem))

(fn ConstructionScript)

(fn TryPickupItem
  (params (InPickableITem :type BP%20Pickable%20Item%20Object%20Reference) (InPlayerState :type Player%20State%20Object%20Reference))
  (Utilities|FlowControl|Sequence
    (:then_0
      (bind _returnvalue (Game|SpawnActorfromClass "/Game/BP/Game/Item/Equip/BP_EquipItem.BP_EquipItem_C" (Math|Transform|MakeTransform "0, 0, 0" "0, 0, 0" "1.000000,1.000000,1.000000") "AdjustIfPossibleButAlwaysSpawn" "MultiplyWithRoot" 0 0))
      (bind _output_get (LocalVariables|SetSpawnEquipItem _returnvalue))
      (Actor|SetOwner _output_get InPlayerState)
      (bind _returnvalue_2 (Utilities|GetDataTableRow "/Game/BP/Game/Datas/Datatable/Item/DT_EquipItemData.DT_EquipItemData" (Variables|/Game/BP/Game/Item/BP_WorldActor_Base.BP_WorldActor_Base_C|GetID InPickableITem))
        (:then
          (LocalVariables|SetLocalSpawnItemData _returnvalue_2))))
    (:then_1
      (Default|Initialize (LocalVariables|GetSpawnEquipItem) (.id (LocalVariables|GetLocalSpawnItemData)) (.itemname (LocalVariables|GetLocalSpawnItemData)) (.staticmesh (LocalVariables|GetLocalSpawnItemData)) "0, 0, 0" (.itemweight (LocalVariables|GetLocalSpawnItemData)) (.damagetype (LocalVariables|GetLocalSpawnItemData)) (.damgevalue (LocalVariables|GetLocalSpawnItemData)) (.icon (LocalVariables|GetLocalSpawnItemData)) "NewEnumerator0" (.movementpanelty (LocalVariables|GetLocalSpawnItemData))))
    (:then_2
      (Actor|DestroyActor InPickableITem)
      (return (LocalVariables|GetSpawnEquipItem)))))

(fn TryDropItem
  (params (InDropItem :type BP%20World%20Actor%20Base%20Object%20Reference) (InDropLocation :type Vector) (InImpluse :type Vector))
  (bind _asbp_equip_item (Utilities|Casting|CastToBP_EquipItem InDropItem))
  (LocalVariables|SetLocalSpawnItemId (Variables|/Game/BP/Game/Item/BP_WorldActor_Base.BP_WorldActor_Base_C|GetID _asbp_equip_item))
  (bind _returnvalue (Game|SpawnActorfromClass "/Game/BP/Game/Item/Pickable/BP_PickableItem.BP_PickableItem_C" (Math|Transform|MakeTransform InDropLocation "0, 0, 0" "1.000000,1.000000,1.000000") "AdjustIfPossibleButAlwaysSpawn" "MultiplyWithRoot" 0 0))
  (LocalVariables|SetSpawnItem _returnvalue)
  (bind _returnvalue_2 (Utilities|GetDataTableRow "/Game/BP/Game/Datas/Datatable/Item/DT_EquipItemData.DT_EquipItemData" (LocalVariables|GetLocalSpawnItemId))
    (:then
      (Default|Initialize (LocalVariables|GetSpawnItem) (.id _returnvalue_2) (.itemname _returnvalue_2) (.staticmesh _returnvalue_2) "0, 0, 0" (.itemweight _returnvalue_2) (.damagetype _returnvalue_2) 0.0 0 "NewEnumerator0" "NewEnumerator0")
      (Actor|DestroyActor InDropItem)
      (Physics|SetSimulatePhysics (Variables|/Game/BP/Game/Item/BP_WorldActor_Base.BP_WorldActor_Base_C|GetBody (LocalVariables|GetSpawnItem)) true)
      (Physics|AddImpulse (Variables|/Game/BP/Game/Item/BP_WorldActor_Base.BP_WorldActor_Base_C|GetBody (LocalVariables|GetSpawnItem)) InImpluse "None" false))))

(fn GenerateWorldItemWeapon
  (Utilities|FlowControl|Sequence
    (:then_0
      (bind _outrownames (DataTable|GetDataTableRowNames "/Game/BP/Game/Datas/Datatable/ItemGenerater/DT_SpawnWeaponLocation.DT_SpawnWeaponLocation"))
      (for _array_element _outrownames
        (bind _returnvalue (Utilities|GetDataTableRow "/Game/BP/Game/Datas/Datatable/ItemGenerater/DT_SpawnWeaponLocation.DT_SpawnWeaponLocation" _array_element)
          (:then
            (LocalVariables|SetLocalItemID (.id _returnvalue))
            (bind _returnvalue_2 (Game|SpawnActorfromClass "/Game/BP/Game/Item/Pickable/BP_PickableItem.BP_PickableItem_C" (Math|Transform|MakeTransform (.location _returnvalue) "0, 0, 0" "1.000000,1.000000,1.000000") "AdjustIfPossibleButAlwaysSpawn" "MultiplyWithRoot" 0 0))
            (LocalVariables|SetLocalSpawnWeaponItem _returnvalue_2)
            (bind _returnvalue_3 (Utilities|GetDataTableRow "/Game/BP/Game/Datas/Datatable/Item/DT_EquipItemData.DT_EquipItemData" (LocalVariables|GetLocalItemID))
              (:then
                (Default|Initialize (LocalVariables|GetLocalSpawnWeaponItem) (.ID (Utilities|Struct|BreakST_EquipItem _returnvalue_3)) (.ItemName (Utilities|Struct|BreakST_EquipItem _returnvalue_3)) (.StaticMesh (Utilities|Struct|BreakST_EquipItem _returnvalue_3)) (.DropRotationOffset (Utilities|Struct|BreakST_EquipItem _returnvalue_3)) 0.0 (.DamageType (Utilities|Struct|BreakST_EquipItem _returnvalue_3)) 0.0 0 "NewEnumerator0" "NewEnumerator0")))))))))

(fn UpdateSocre
  (params (NewBreakItem :type BP%20Break%20Actor%20Base%20Object%20Reference))
  (if (Utilities|Set|Contains (Variables|Score|GetBreakItemList) NewBreakItem)
    (Variables|Score|SetZoneScore (- (Variables|Score|GetZoneScore) (Variables|/Game/BP/Game/BreakActor/BP_BreakActor_Base.BP_BreakActor_Base_C|GetBsaeScore NewBreakItem)))
    (Utilities|Set|Remove (Variables|Score|GetBreakItemList) NewBreakItem)
    (else
      (Utilities|Set|Add (Variables|Score|GetBreakItemList) NewBreakItem)
      (bind _valuepin (Utilities|Set|ForEachLoop(Set) (Variables|Score|GetBreakItemList))
        (:then
          (LocalVariables|SetCurrentSocore (+ (LocalVariables|GetCurrentSocore) (Variables|/Game/BP/Game/BreakActor/BP_BreakActor_Base.BP_BreakActor_Base_C|GetBsaeScore _valuepin))))
        (:CompletedPin
          (Variables|Score|SetZoneScore (LocalVariables|GetCurrentSocore)))))))

(fn UpdateGameTimer
  (Math|Float|DecrementFloat (Variables|Time|GetRemainingTime)
    (:%20%20
      (if (>= (Variables|Time|GetRemainingTime) 0.0)
        (bind _asbp_game_state (Utilities|Casting|CastToBP_GameState (Game|GetGameState)))
        (Default|S2MUpdateGameTimer _asbp_game_state (Variables|Time|GetRemainingTime))
        (else
          (CallFunction|GameOver))))))

(fn UpdateBreakScore
  (Math|Integer|IncrementInt (Variables|Score|GetBreakObjectAmount)
    (:%20%20
      (Variables|Score|SetBreakBonusScore (+ (Variables|Score|GetBreakBonusScore) (Variables|Score|GetBreakObjectScore))))))

(fn CalculateRank
  (LocalVariables|SetCurrentModifier (/ (Math|Conversions|ToFloat(Integer) (+ (Variables|Score|GetZoneScore) (Variables|Score|GetBreakBonusScore))) (Math|Conversions|ToFloat(Integer) (Variables|Score|GetGoalScore))))
  (bind _outrownames (DataTable|GetDataTableRowNames "/Game/BP/Game/Datas/Datatable/Score/DT_ScoreGrade.DT_ScoreGrade"))
  (bind _array_element (Utilities|Array|ForEachLoopwithBreak _outrownames :!label _label)
    (:LoopBody
      (bind _returnvalue (Utilities|GetDataTableRow "/Game/BP/Game/Datas/Datatable/Score/DT_ScoreGrade.DT_ScoreGrade" _array_element)
        (:then
          (if (>= (LocalVariables|GetCurrentModifier) (.modifier _returnvalue))
            (Variables|Score|SetRank (.rank _returnvalue))
            (goto _label Break)))))))