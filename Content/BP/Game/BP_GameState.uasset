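; BP_GameState is the game state that relays the match timer, game-over state and result data to local players.
; S2M_UpdateGameTimer passes the remaining time to the first BP_PlayerController to handle.
; The bIsGameOver RepNotify tells that controller's BP_HUD to show the result UI.
; SetResultInfo stores the result rank plus goal, zone and break scores, along with the break count.
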(event Custom|S2M_UpdateGameTimer
  (params (InRemainingTime :type Float%20%28double-precision%29))
  (bind _asbp_player_controller (Utilities|Casting|CastToBP_PlayerController (Game|GetPlayerController 0)))
  (Default|HandleUpdateGameTImer _asbp_player_controller InRemainingTime))

(fn ConstructionScript)

(fn OnRepBIsGameOver
  (bind _asbp_hud (Utilities|Casting|CastToBP_HUD (HUD|GetHUD (Game|GetPlayerController 0))))
  (Default|ShowResultUI _asbp_hud))

(fn SetResultInfo
  (params (ResultRank :type String) (GoalScore :type Integer) (ZoneScore :type Integer) (BreakCount :type Integer) (BreakScore :type Integer))
  (Variables|Default|SetResult%20Rank ResultRank)
  (Variables|Default|SetGoal%20Score GoalScore)
  (Variables|Default|SetZone%20Score ZoneScore)
  (Variables|Default|SetBreak%20Count BreakCount)
  (Variables|Default|SetBreak%20Score BreakScore))