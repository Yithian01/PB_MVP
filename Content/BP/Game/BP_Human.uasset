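; Human character Blueprint that turns damage into a stun, dropping the character into a physics ragdoll and later standing it back up.
; AnyDamage feeds BPCStunSystem: a stun starts the ragdoll and a timeline refilling HP, while other hits start a timed invulnerability window.
; When the timeline ends, hits are re-enabled and recovery restores the cached mesh transform, collision and walking.
; Ragdoll start and recovery route through S2M-prefixed RPC events.
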(event Custom|OnEnableHit
  ;[0.15 0.15 0.15 0.5] Enhanced AnyDamage
  (CallFunction|DamgeEnable))

(event EventBeginPlay
  ;[0.15 0.15 0.15 0.5] Initialize
  (Variables|Default|SetOriginTransform (Transformation|GetRelativeTransform (Variables|Character|GetMesh))))

(event Game|Damage|EventAnyDamage
  (params (Damage :type Float%20%28single-precision%29) (DamageType :type Damage%20Type%20Object%20Reference) (InstigatedBy :type Controller%20Object%20Reference) (DamageCauser :type Actor%20Object%20Reference))
  ;[0.15 0.15 0.15 0.5] Enhanced AnyDamage
  (if (and (Variables|Default|GetbIsEnableHit) (not (Variables|Default|GetbIsRegdoll)))
    (Variables|Default|SetbIsEnableHit false)
    (bind _bisstun (Default|TakeDamage (Variables|Default|GetBPC_StunSystem) Damage))
    (if _bisstun
      (CallFunction|S2MStartRedoll)
      (bind _alpha (Timeline|Timeline_0 PlayFromStart)
        (:Update
          (Default|RecoverHp (Variables|Default|GetBPC_StunSystem) (Math|Float|Lerp 0.0 (Variables|/Game/BP/Game/Components/StatAttributeComponent/BPC_StunSystem.BPC_StunSystem_C|GetMaxHp (Variables|Default|GetBPC_StunSystem)) _alpha)))
        (:Finished
          (CallFunction|DamgeEnable)
          (CallFunction|S2MRecoveryRegdoll)))
      (else
        (Utilities|Time|SetTimerbyEvent (delegate Custom|OnEnableHit) 2.0)))))

(event Custom|S2M_RecoveryRegdoll
  ;[0.15 0.15 0.15 0.5] Regdoll
  (Regdoll|RecoveryRegdoll))

(event Custom|S2M_StartRedoll
  ;[0.15 0.15 0.15 0.5] Regdoll
  (Regdoll|StartRegdoll))

(fn ConstructionScript)

(fn StartRegdoll
  (Utilities|FlowControl|Sequence
    (:then_0
      (Variables|Default|SetbIsRegdoll true)
      (Pawn|Components|CharacterMovement|DisableMovement (Variables|Character|GetCharacterMovement)))
    (:then_1
      (Collision|SetCollisionEnabled (Variables|Collision|GetCapsuleComponent) "NoCollision")
      (Collision|SetCollisionEnabled (Variables|Character|GetMesh) "QueryAndPhysics"))
    (:then_2
      (Physics|SetSimulatePhysics (Variables|Character|GetMesh) true))))

(fn RecoveryRegdoll
  (Utilities|FlowControl|Sequence
    (:then_0
      (Physics|SetSimulatePhysics (Variables|Character|GetMesh) false))
    (:then_1
      (Transformation|SetRelativeRotation (Variables|Character|GetMesh) (Math|Rotator|MakeRotator 0.0 0.0 (.yaw (Transformation|GetActorRotation))) false false)
      (Transformation|SetRelativeTransform (Variables|Character|GetMesh) (Variables|Default|GetOriginTransform) false false))
    (:then_3
      (Collision|SetCollisionEnabled (Variables|Collision|GetCapsuleComponent) "QueryAndPhysics")
      (Collision|SetCollisionEnabled (Variables|Character|GetMesh) "NoCollision"))
    (:then_4
      (Pawn|Components|CharacterMovement|SetMovementMode (Variables|Character|GetCharacterMovement) "MOVE_Walking" 0)
      (Variables|Default|SetbIsRegdoll false))))

(fn DamgeEnable
  (Variables|Default|SetbIsEnableHit true))

(fn OnHealthChanged
  (params (CurrentHp :type Float%20%28double-precision%29) (MaxHp :type Float%20%28double-precision%29)))