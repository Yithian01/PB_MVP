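; Breakable-object component that tracks an object's health and armor type, set through Initialize along with the Geometry Collection used as its broken form.
; ProcessPointDamage scales the player's equipped-item damage, or an unarmed default, by a DT_DamageModifier row keyed on damage and armor type, then reports breakage and damage dealt.
; CheckHit separately decrements MaxHP for one damage type and, at zero, spawns the Geometry Collection with an impulse at the impact point.
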(event EventBeginPlay)

(fn CheckHit
  (params (DamageType :type E_DamageType%20Enum :default "NewEnumerator0") (ActorTransfrom :type Transform) (ImpactPoint :type Vector) (impactForce :type Vector))
  (if (Utilities|Enum|Equal(Enum) DamageType "NewEnumerator1")
    (if (<= (- (Variables|Default|GetMaxHP) 1) 0)
      (CallFunction|SpawnGCObject ActorTransfrom ImpactPoint impactForce)
      (return true)
      (else
        (Variables|Default|SetMaxHP (Math|Conversions|ToFloat(Integer) (- (Variables|Default|GetMaxHP) 1)))
        (return false)))
    (else
      (return false))))

(fn SpawnGCObject
  (params (SpawnTransfrom :type Transform) (ImpactPoint :type Vector) (ImpactForce :type Vector))
  (bind _returnvalue (Game|SpawnActorfromClass "/Script/GeometryCollectionEngine.GeometryCollectionActor" SpawnTransfrom "AlwaysSpawn" "MultiplyWithRoot" 0 0))
  (bind _output_get (LocalVariables|SetSpawnActor (Variables|/Script/GeometryCollectionEngine.GeometryCollectionActor|GetGeometryCollectionComponent _returnvalue)))
  (Class|GeometryCollectionComponent|SetRestCollection _output_get (Variables|Default|GetConvert_GC) true)
  (Physics|AddImpulseatLocation (LocalVariables|GetSpawnActor) ImpactForce ImpactPoint "None")
  (Collision|SetCollisionEnabled (LocalVariables|GetSpawnActor) "QueryOnly"))

(fn Initialize
  (params (Convert_GC :type Geometry%20Collection%20Object%20Reference) (ArmorType :type E_ArmorType%20Enum :default "NewEnumerator0") (CurrentHp :type Float%20%28double-precision%29) (MaxHp :type Float%20%28double-precision%29))
  (Variables|Default|SetConvert_GC Convert_GC)
  (Variables|Default|SetArmorType ArmorType)
  (Variables|Default|SetCurrentHP CurrentHp)
  (Variables|Default|SetMaxHP MaxHp))

(fn ProcessPointDamage
  (params (DamageCursor :type Actor%20Object%20Reference))
  (Utilities|FlowControl|Sequence
    (:then_0
      (bind _asbp_player (Utilities|Casting|CastToBP_Player DamageCursor))
      (bind _output_get (LocalVariables|SetLocalEquipItem (Variables|/Game/BP/Game/Player/BP_Player.BP_Player_C|GetEquippedItem _asbp_player)))
      (Utilities|IsValid _output_get
        (:Is%20Valid
          (LocalVariables|SetLocalDamageValue (Variables|/Game/BP/Game/Item/BP_WorldActor_Base.BP_WorldActor_Base_C|GetDamageValue (LocalVariables|GetLocalEquipItem))))
        (:Is%20Not%20Valid
          (LocalVariables|SetLocalDamageValue 1e+01))))
    (:then_1
      (bind _output_get_2 (LocalVariables|SetLocalFinalDamage (* (LocalVariables|GetLocalDamageValue) (CallFunction|GetDamgeModifier (LocalVariables|GetLocalEquipItem)))))
      (bind _bisbreak (CallFunction|ApplyDamage _output_get_2))
      (return _bisbreak (LocalVariables|GetLocalFinalDamage)))))

(fn GetDamgeModifier
  (params (InEquipItem :type BP%20World%20Actor%20Base%20Object%20Reference))
  (Utilities|FlowControl|Sequence
    (:then_0
      (Utilities|IsValid InEquipItem
        (:Is%20Valid
          (LocalVariables|SetLocalDamageType (Utilities|String|EnumtoString (Variables|/Game/BP/Game/Item/BP_WorldActor_Base.BP_WorldActor_Base_C|GetDamgeType InEquipItem))))
        (:Is%20Not%20Valid
          (LocalVariables|SetLocalDamageType (Utilities|String|EnumtoString (Utilities|Enum|LiteralenumE_DamageType "NewEnumerator2"))))))
    (:then_1
      (bind _returnvalue (Utilities|GetDataTableRow "/Game/BP/Game/Datas/Datatable/Item/DT_DamageModifier.DT_DamageModifier" (Utilities|String|StringToName (Utilities|String|Append (LocalVariables|GetLocalDamageType) "_" (Utilities|String|EnumtoString (Variables|Default|GetArmorType)))))
        (:then
          (return (.modifier _returnvalue)))))))

(fn ApplyDamage
  (params (InApplyDamage :type Float%20%28double-precision%29))
  (bind _output_get (LocalVariables|SetLocalIsBreak (<= (- (Variables|Default|GetCurrentHP) InApplyDamage) 0.0)))
  (if _output_get
    (Variables|Default|SetCurrentHP 0.0)
    (return (LocalVariables|GetLocalIsBreak))
    (else
      (Variables|Default|SetCurrentHP (- (Variables|Default|GetCurrentHP) InApplyDamage))
      (return (LocalVariables|GetLocalIsBreak)))))