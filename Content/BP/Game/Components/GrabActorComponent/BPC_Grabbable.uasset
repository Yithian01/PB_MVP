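; BPC_Grabbable is a component that tracks whether something can be grabbed and what is currently grabbing it.
; CanGrab passes only while it is grabbable and not already held, Grab and Release set or clear the grabber and held flag, and SetGrabable toggles availability.
; It only stores state: Grab does not check CanGrab itself, and no attachment, physics or event logic runs here.
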(event EventBeginPlay)

(fn CanGrab
  (return (and (Variables|Default|GetbIsGrabable) (not (Variables|Default|GetbIsGrabbed)))))

(fn Grab
  (params (Grabber :type Actor%20Object%20Reference))
  (Variables|Default|SetCurrentGrabber Grabber)
  (Variables|Default|SetbIsGrabbed true))

(fn Release
  (Variables|Default|SetCurrentGrabber 0)
  (Variables|Default|SetbIsGrabbed false))

(fn SetGrabable
  (params (NewState :type Boolean))
  (Variables|Default|SetbIsGrabable NewState))