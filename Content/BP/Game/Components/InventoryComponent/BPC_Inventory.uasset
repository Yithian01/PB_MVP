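; Inventory component that manages a fixed set of quick slots for carried items and tracks the selected slot.
; Adding fills the first empty slot, swapping pickables for equip items through BP_GameMode, then hides the item and returns an attach socket.
; Removing hands equip items to the GameMode or detaches and impulses others, then clears the selected slot.
; S2C events relay slot changes to UI; movement penalties are summed from a DataTable.
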(event EventBeginPlay)

(event Custom|S2C_ChangeSlot
  (params (InOldIndex :type Integer) (InNewIndex :type Integer))
  ;[0.15 0.15 0.15 0.5] QuickSlot & UI
  (Default|CallOnSelectQuickSlot InOldIndex InNewIndex))

(event Custom|S2C_UpdateQuickSlotUI
  (params (InIndex :type Integer) (ItemIcon :type Texture%202D%20Object%20Reference))
  ;[0.15 0.15 0.15 0.5] QuickSlot & UI
  (Default|CallOnUpdateItem InIndex ItemIcon))

(fn TryAddItem
  (params (AddItem :type BP%20World%20Actor%20Base%20Object%20Reference) (InPlayerState :type Player%20State%20Object%20Reference))
  (bind (_addindex _bisplace) (CallFunction|TryGetPlaceIndex))
  (if _bisplace
    (LocalVariables|SetLocalAddIndex _addindex)
    (bind _asbp_pickable_item (Utilities|Casting|CastToBP_PickableItem AddItem)
      (:then
        (LocalVariables|SetLocalPickableItem _asbp_pickable_item)
        (bind _asbp_game_mode (Utilities|Casting|CastToBP_GameMode (Game|GetGameMode)))
        (bind _spawnitem (Default|TryPickupItem _asbp_game_mode (LocalVariables|GetLocalPickableItem) InPlayerState))
        (LocalVariables|SetLocalEquipItem _spawnitem)
        (Utilities|Array|SetArrayElem (Variables|Default|GetItems) (LocalVariables|GetLocalAddIndex) (LocalVariables|GetLocalEquipItem))
        (CallFunction|S2CUpdateQuickSlotUI (LocalVariables|GetLocalAddIndex) (Variables|/Game/BP/Game/Item/BP_WorldActor_Base.BP_WorldActor_Base_C|GetItemIcon (LocalVariables|GetLocalEquipItem)))
        (Default|S2MinQuickSlotCollisionPreset (LocalVariables|GetLocalEquipItem))
        (Rendering|SetActorHiddenInGame (LocalVariables|GetLocalEquipItem) true)
        (return (LocalVariables|GetLocalEquipItem) "HandGrip_R"))
      (:CastFailed
        (Utilities|Array|SetArrayElem (Variables|Default|GetItems) (LocalVariables|GetLocalAddIndex) AddItem)
        (CallFunction|S2CUpdateQuickSlotUI (LocalVariables|GetLocalAddIndex) (Variables|/Game/BP/Game/Item/BP_WorldActor_Base.BP_WorldActor_Base_C|GetItemIcon AddItem))
        (Default|S2MinQuickSlotCollisionPreset AddItem)
        (Rendering|SetActorHiddenInGame AddItem true)
        (return AddItem "GrabSocket")))))

(fn TryGetPlaceIndex
  (for (_array_element _array_index) (Variables|Default|GetItems)
    (Utilities|IsValid _array_element
      (:Is%20Not%20Valid
        (return _array_index true))))
  (return -1 false))

(fn TryRemoveEquipItem
  (params (InDropItem :type BP%20World%20Actor%20Base%20Object%20Reference) (InDropLocation :type Vector) (InImpluse :type Vector))
  (Utilities|FlowControl|Sequence
    (:then_0
      (Utilities|Casting|CastToBP_EquipItem InDropItem
        (:then
          (bind _asbp_game_mode (Utilities|Casting|CastToBP_GameMode (Game|GetGameMode)))
          (Default|TryDropItem _asbp_game_mode InDropItem InDropLocation InImpluse))
        (:CastFailed
          (Transformation|DetachFromActor InDropItem "KeepWorld" "KeepWorld" "KeepWorld")
          (Default|S2MBreakActorCollisionPresst InDropItem)
          (Physics|AddImpulse (Variables|/Game/BP/Game/Item/BP_WorldActor_Base.BP_WorldActor_Base_C|GetBody InDropItem) InImpluse "None" false))))
    (:then_1
      (LocalVariables|SetEmptyItem 0)
      (Utilities|Array|SetArrayElem (Variables|Default|GetItems) (Variables|Default|GetCurrentSelectIndex) (LocalVariables|GetEmptyItem))
      (CallFunction|S2CUpdateQuickSlotUI (Variables|Default|GetCurrentSelectIndex)))))

(fn SelectSlot
  (params (NewSlot :type Integer))
  (LocalVariables|SetLocalOldIndex (Variables|Default|GetCurrentSelectIndex))
  (bind _output_get (Variables|Default|SetCurrentSelectIndex (Math|Integer|Clamp(Integer) (+ NewSlot (Variables|Default|GetCurrentSelectIndex)) 0 (- (Variables|Default|GetMaxIndex) 1))))
  (CallFunction|S2CChangeSlot (LocalVariables|GetLocalOldIndex) _output_get)
  (return (Utilities|Array|Get(acopy) (Variables|Default|GetItems) _output_get)))

(fn GetCalculateMovementPenalty
  (for _array_element (Variables|Default|GetItems)
    (Utilities|IsValid _array_element
      (:Is%20Valid
        (bind _returnvalue (Utilities|GetDataTableRow "/Game/BP/Game/Datas/Datatable/Item/DT_MovementPenalty.DT_MovementPenalty" (Utilities|Name|EnumtoName (Variables|/Game/BP/Game/Item/BP_WorldActor_Base.BP_WorldActor_Base_C|GetMovement%20Penalty _array_element)))
          (:then
            (LocalVariables|SetLocalMovementPenalty (+ (.penalty _returnvalue) (LocalVariables|GetLocalMovementPenalty))))))))
  (return (LocalVariables|GetLocalMovementPenalty)))