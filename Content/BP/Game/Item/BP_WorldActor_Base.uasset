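; Base world actor for items, holding item data (identity, mesh, icon, weight, damage, armor and movement penalty) around a Body mesh component.
; Initialize copies the passed data into variables and applies the mesh to Body, though RotationOffset goes unused.
; Outline events toggle Body's custom depth when enabled, and Interact is an empty hook.
; S2M events switch collision profiles for quick-slot and broken states, the latter also enabling physics and clearing the outline.
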(event EventBeginPlay)

(event EventTurnOffOutline
  (if (Variables|Default|GetbIsEnableOutline)
    (Rendering|SetRenderCustomDepth (Variables|Default|GetBody) false)))

(event EventTurnonOutline
  (if (Variables|Default|GetbIsEnableOutline)
    (Rendering|SetRenderCustomDepth (Variables|Default|GetBody) true)))

(event EventInteract
  (params (InPlayerRef :type BP%20Player%20Object%20Reference)))

(event Custom|S2M_BreakActorCollisionPresst
  (Collision|SetCollisionProfileName (Variables|Default|GetBody) "BreakActor" false :!class /Script/Engine.PrimitiveComponent)
  (Physics|SetSimulatePhysics (Variables|Default|GetBody) true)
  (Rendering|SetRenderCustomDepth (Variables|Default|GetBody) false))

(event Custom|S2M_InQuickSlotCollisionPreset
  (Collision|SetCollisionProfileName (Variables|Default|GetBody) "InQuickSlot" false :!class /Script/Engine.PrimitiveComponent))

(fn ConstructionScript)

(fn Initialize
  (params (ID :type Name) (ItemName :type Text) (StaticMesh :type Static%20Mesh%20Object%20Reference) (RotationOffset :type Rotator) (ItemWeight :type Float%20%28double-precision%29) (DamgeType :type E_DamageType%20Enum :default "NewEnumerator1") (DamageValue :type Float%20%28double-precision%29) (Icon :type Texture%202D%20Object%20Reference) (ArmorType :type E_ArmorType%20Enum :default "NewEnumerator0") (MovementPenalty :type E_MovementPenalty%20Enum :default "NewEnumerator0"))
  (Variables|Default|SetID ID)
  (Variables|Default|SetItemName ItemName)
  (Components|StaticMesh|SetStaticMesh (Variables|Default|GetBody) StaticMesh)
  (Variables|Default|SetStaticMesh StaticMesh)
  (Variables|Default|SetItemWeight ItemWeight)
  (Variables|Default|SetDamgeType DamgeType)
  (Variables|Default|SetDamageValue DamageValue)
  (Variables|Default|SetItemIcon Icon)
  (Variables|Default|SetArmorType ArmorType)
  (Variables|Default|SetMovement%20Penalty MovementPenalty))