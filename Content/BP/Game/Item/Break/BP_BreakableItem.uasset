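; BP_BreakableItem is a pickup item Blueprint for breakable items, though it contains no breaking logic of its own.
; It enables outlining on BeginPlay and Initialize, toggling custom depth rendering on its Body for the highlight.
; Interact runs the parent logic, then passes itself to the player's pickup handler if that player is valid.
; Initialize forwards item data to the parent, except the RotationOffset input, which is not passed on.
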(event EventBeginPlay
  (Variables|Default|SetbIsEnableOutline true))

(event EventInteract
  (params (InPlayerRef :type BP%20Player%20Object%20Reference))
  (|CallParentFunction InPlayerRef)
  (Utilities|IsValid InPlayerRef
    (:Is%20Valid
      (Default|HandlePickupItme InPlayerRef self))))

(event EventTurnOffOutline
  (if (Variables|Default|GetbIsEnableOutline)
    (Rendering|SetRenderCustomDepth (Variables|Default|GetBody) false)))

(event EventTurnonOutline
  (if (Variables|Default|GetbIsEnableOutline)
    (Rendering|SetRenderCustomDepth (Variables|Default|GetBody) true)))

(fn ConstructionScript)

(fn Initialize
  (params (ID :type Name :default "None") (ItemName :type Text) (StaticMesh :type Static%20Mesh%20Object%20Reference) (RotationOffset :type Rotator :default "0, 0, 0") (ItemWeight :type Float%20%28double-precision%29) (DamgeType :type E_DamageType%20Enum :default "NewEnumerator1") (DamageValue :type Float%20%28double-precision%29) (Icon :type Texture%202D%20Object%20Reference) (ArmorType :type E_ArmorType%20Enum :default "NewEnumerator0"))
  (|CallParentFunction ID ItemName StaticMesh "0, 0, 0" ItemWeight DamgeType DamageValue Icon ArmorType)
  (Variables|Default|SetbIsEnableOutline true))