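; BP_Barrel is a barrel prop, filed among breakable item props, that can show an outline.
; Its outline on and off events toggle custom depth rendering on the Body component, gated by the IsEnableOutline flag.
; BeginPlay and the construction script only call the parent, so the file itself adds no breaking logic.
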(event EventBeginPlay
  (|CallParentFunction))

(event EventTurnOffOutline
  (if (Variables|Default|GetbIsEnableOutline)
    (Rendering|SetRenderCustomDepth (Variables|Default|GetBody) false)))

(event EventTurnonOutline
  (if (Variables|Default|GetbIsEnableOutline)
    (Rendering|SetRenderCustomDepth (Variables|Default|GetBody) true)))

(fn ConstructionScript
  (|CallParentFunction))