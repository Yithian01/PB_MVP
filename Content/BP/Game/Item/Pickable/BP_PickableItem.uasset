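; BP_PickableItem is an item Blueprint that the player can pick up by interacting with it.
; Interact runs the parent logic, then passes the item to the player's HandlePickupItme if that player reference is valid.
; Initialize applies a rotation offset to the Body, forwards the item data to the parent and enables outlining.
; The outline events then toggle Custom Depth rendering on the Body.
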(event EventBeginPlay)

(event EventTurnonOutline
  ;[0.15 0.15 0.15 0.5] Outline
  (if (Variables|Default|GetbIsEnableOutline)
    (Rendering|SetRenderCustomDepth (Variables|Default|GetBody) true)))

(event EventTurnOffOutline
  ;[0.15 0.15 0.15 0.5] Outline
  (if (Variables|Default|GetbIsEnableOutline)
    (Rendering|SetRenderCustomDepth (Variables|Default|GetBody) false)))

(event EventInteract
  (params (InPlayerRef :type BP%20Player%20Object%20Reference))
  ;[0.15 0.15 0.15 0.5] Interaction
  (|CallParentFunction InPlayerRef)
  (Utilities|IsValid InPlayerRef
    (:Is%20Valid
      (Default|HandlePickupItme InPlayerRef self))))

(fn ConstructionScript)

(fn Initialize
  (params (ID :type Name :default "None") (ItemName :type Text) (StaticMesh :type Static%20Mesh%20Object%20Reference) (RotationOffset :type Rotator :default "0, 0, 0") (ItemWeight :type Float%20%28double-precision%29) (DamgeType :type E_DamageType%20Enum :default "NewEnumerator1") (DamageValue :type Float%20%28double-precision%29) (Icon :type Texture%202D%20Object%20Reference) (ArmorType :type E_ArmorType%20Enum :default "NewEnumerator0") (MovementPenalty :type E_MovementPenalty%20Enum :default "NewEnumerator0"))
  (Transformation|SetRelativeRotation (Variables|Default|GetBody) RotationOffset false false)
  (|CallParentFunction ID ItemName StaticMesh "0, 0, 0" ItemWeight DamgeType DamageValue Icon ArmorType MovementPenalty)
  (Variables|Default|SetbIsEnableOutline true))