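; Base actor for world items, holding identity, display data and a static mesh body that can be dropped or thrown.
; Init functions store spawn ID/SN and item type, name, UI prefix, icon, mesh and outline eligibility.
; Dropping enables physics with linear and angular impulses; when Body sleeps, it blocks Pawns and reattaches after the root snaps to its transform.
; Outlines toggle through custom depth rendering when allowed.
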(event OnComponentSleep(Body)
  (params (SleepingComponent :type Primitive%20Component%20Object%20Reference) (BoneName :type Name :default "None"))
  (Collision|SetCollisionResponsetoChannel (Variables|Default|GetBody) "ECC_Pawn" "ECR_Block")
  (Transformation|SetRelativeTransform (Variables|Default|GetDefaultSceneRoot) (Transformation|GetWorldTransform (Variables|Default|GetBody)) false false)
  (Transformation|AttachComponentToComponent (Variables|Default|GetBody) (Variables|Default|GetDefaultSceneRoot) "None" "KeepWorld" "KeepWorld" "KeepWorld" false))

(event Custom|OnDropItem
  (params (ThrowImpulse :type Vector))
  (Physics|SetSimulatePhysics (Variables|Default|GetBody) true)
  (Physics|AddImpulse (Variables|Default|GetBody) ThrowImpulse "None" false)
  (Class|PrimitiveComponent|AddAngularImpulseinRadians (Variables|Default|GetBody) ThrowImpulse "None" false))

(event EventBeginPlay
  (|CallParentFunction))

(event Collision|EventActorBeginOverlap
  (params (OtherActor :type Actor%20Object%20Reference))
  (|CallParentFunction OtherActor) ; This node is disabled and will not be called.\nDrag off pins to build functionality.
)

(event EventTick
  (params (DeltaSeconds :type Float%20%28single-precision%29))
  (|CallParentFunction DeltaSeconds) ; This node is disabled and will not be called.\nDrag off pins to build functionality.
)

(fn ConstructionScript
  (|CallParentFunction))

(fn InitializeSpawnData
  (params (ID :type Name) (SN :type String))
  (Variables|Default|SetID ID)
  (Variables|Default|SetSN SN))

(fn InitializeWorldItemBaseData
  (params (ItemType :type E_ItemType%20Enum :default "NewEnumerator0") (ItemName :type Text) (UIPrefix :type E_UIPrefix%20Enum :default "NewEnumerator0") (StaticMesh :type Static%20Mesh%20Object%20Reference) (Icon :type Texture%202D%20Object%20Reference) (OutlineAble :type Boolean))
  (Utilities|FlowControl|Sequence
    (:then_0
      (Variables|Default|SetItemType ItemType))
    (:then_1
      (Variables|Default|SetItemName ItemName))
    (:then_2
      (Variables|Default|SetUIPrefix UIPrefix))
    (:then_3
      (Components|StaticMesh|SetStaticMesh (Variables|Default|GetBody) StaticMesh))
    (:then_4
      (Variables|Default|SetIcon Icon))
    (:then_5
      (Variables|Default|SetbIsOutlineAble OutlineAble))))

(fn EnableOutline
  (params (bIsEnable :type Boolean))
  (if (Variables|Default|GetbIsOutlineAble)
    (Rendering|SetRenderCustomDepth (Variables|Default|GetBody) bIsEnable)))

(fn SetOutlineAble
  (params (Value :type Boolean))
  (Variables|Default|SetbIsOutlineAble Value))