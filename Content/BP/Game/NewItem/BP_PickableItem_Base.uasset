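; Base actor for pickable items that a player can collect by interacting with it.
; Initialize stores the item's ID, type, name and icon, sets the Body mesh and rotation offset, and enables outlining.
; Outline events toggle custom depth rendering on Body while outlining is enabled.
; Interact runs the parent logic, then passes the item to a valid player reference's pickup handler.
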(event EventBeginPlay)

(event Collision|EventActorBeginOverlap
  (params (OtherActor :type Actor%20Object%20Reference)))

(event EventTick
  (params (DeltaSeconds :type Float%20%28single-precision%29)))

(event EventTurnonOutline
  (if (Variables|Default|GetbIsEnableOutline)
    (Rendering|SetRenderCustomDepth (Variables|Default|GetBody) true)))

(event EventTurnOffOutline
  (if (Variables|Default|GetbIsEnableOutline)
    (Rendering|SetRenderCustomDepth (Variables|Default|GetBody) false)))

(event EventInteract
  (params (InPlayerRef :type BP%20Player%20Object%20Reference))
  (|CallParentFunction InPlayerRef)
  (Utilities|IsValid InPlayerRef
    (:Is%20Valid
      (Default|HandlePickupItme InPlayerRef self))))

(fn ConstructionScript)

(fn Initialize
  (params (ID :type Name) (ItemType :type E_ItemType%20Enum :default "NewEnumerator0") (ItemName :type Text) (StaticMesh :type Static%20Mesh%20Object%20Reference) (RotationOffset :type Rotator) (ItemIcon :type Texture%202D%20Object%20Reference))
  (Variables|Default|SetID ID)
  (Variables|Default|SetItemType ItemType)
  (Variables|Default|SetItem%20Name ItemName)
  (Components|StaticMesh|SetStaticMesh (Variables|Default|GetBody) StaticMesh)
  (Transformation|SetRelativeRotation (Variables|Default|GetBody) RotationOffset false false)
  (Variables|Default|SetItemIcon ItemIcon)
  (Variables|Default|SetbIsEnableOutline true))