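; BP_PlayerController is the player controller that routes gameplay input to the BP_Player character.
; On BeginPlay it sets game-only input with a hidden cursor, caches the player character and adds the default Enhanced Input mapping context for the local player.
; Input actions call the character's quick slot, pickup, drop, grab and crouch pose-transition functions.
; A separate function forwards the remaining game time to BP_HUD for the timer display.
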(event EventBeginPlay
  (Utilities|FlowControl|Sequence
    (:then_0
      (Variables|Default|SetbShowMouseCursor false)
      (Input|SetInputModeGameOnly self true))
    (:then_1
      (bind _asbp_player (Utilities|Casting|CastToBP_Player (Game|GetPlayerCharacter 0)))
      (Variables|Default|SetPlayerRef _asbp_player))
    (:then_2
      (if (Pawn|IsLocalPlayerController)
        (Input|AddMappingContext (PlayerController|LocalPlayerSubsystems|GetEnhancedInputLocalPlayerSubsystem) "/Game/BP/Game/Input/IMC_Default.IMC_Default" 0 "(bIgnoreAllPressedKeysUntilRelease=True,bForceImmediately=False,bNotifyUserSettings=False)")))))

(event Input|ActionEvents|InputActionPickUp
  (params (Key :type Key%20Structure :default "None"))
  ;[0.15 0.15 0.15 0.5] PickUp Item
  (:Pressed
    (Default|PickUpItem (Variables|Default|GetPlayerRef))))

(event Input|ActionEvents|InputActionDropItem
  (params (Key :type Key%20Structure :default "None"))
  ;[0.15 0.15 0.15 0.5] Drop Item
  (:Pressed
    (Default|DropItem (Variables|Default|GetPlayerRef))))

(event Input|ActionEvents|InputActionQuickSlot_1
  (params (Key :type Key%20Structure :default "None"))
  ;[0.15 0.15 0.15 0.5] QuickSlot
  (:Pressed
    (Default|SelectQuickSlot (Variables|Default|GetPlayerRef))))

(event Input|ActionEvents|InputActionQuickSlot_2
  (params (Key :type Key%20Structure :default "None"))
  ;[0.15 0.15 0.15 0.5] QuickSlot
  (:Pressed
    (Default|SelectQuickSlot (Variables|Default|GetPlayerRef) 1)))

(event Input|ActionEvents|InputActionQuickSlot_3
  (params (Key :type Key%20Structure :default "None"))
  ;[0.15 0.15 0.15 0.5] QuickSlot
  (:Pressed
    (Default|SelectQuickSlot (Variables|Default|GetPlayerRef) 2)))

(event Input|ActionEvents|InputActionCrouch
  (params (Key :type Key%20Structure :default "None"))
  ;[0.15 0.15 0.15 0.5] Pose State
  (:Pressed
    (bind _newparam (Default|TryGetPoseTransition (Variables|Default|GetPlayerRef) "NewEnumerator1"))
    (Default|UpdatePoseState (Variables|Default|GetPlayerRef) _newparam)))

(event Input|ActionEvents|InputActionGrab
  (params (Key :type Key%20Structure :default "None"))
  ;[0.15 0.15 0.15 0.5] Pose State
  (:Pressed
    (Default|ToggleGrab (Variables|Default|GetPlayerRef))))

(fn ConstructionScript)

(fn HandleUpdateGameTImer
  (params (InRemainingTime :type Float%20%28double-precision%29))
  (bind _asbp_hud (Utilities|Casting|CastToBP_HUD (HUD|GetHUD)))
  (Default|UpdateGameTimer _asbp_hud InRemainingTime))