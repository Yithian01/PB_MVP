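; BP_PlayerState is a player state Blueprint that triggers the owning player's widget update when play begins.
; On BeginPlay it casts its pawn to BP_Player and calls TryUpdatePlayerWidget.
; If the cast fails, it retries every 0.2 seconds until the pawn is available, printing a long-lived debug success or failure message on each attempt.
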(event EventBeginPlay
  (bind _self self)
  (bind _returnvalue (Utilities|GetDisplayName _self))
  (bind _asbp_player (Utilities|Casting|CastToBP_Player (PlayerState|GetPawn self) :!label _label)
    (:then
      (Default|TryUpdatePlayerWidget _asbp_player)
      (Development|PrintString (Utilities|String|ToString(Text) (Utilities|Text|FormatText "BP_PlayerState:: {0} 성공" _returnvalue)) true true "(R=0.000000,G=0.660000,B=1.000000,A=1.000000)" 9999.0))
    (:CastFailed
      (Development|PrintString (Utilities|String|ToString(Text) (Utilities|Text|FormatText "BP_PlayerState:: {0} 실패" _returnvalue)) true true "(R=0.000000,G=0.660000,B=1.000000,A=1.000000)" 9999.0)
      (Utilities|FlowControl|Delay 0.2)
      (goto _label))))

(fn ConstructionScript)