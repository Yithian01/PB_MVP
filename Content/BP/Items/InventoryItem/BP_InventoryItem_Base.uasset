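; BP_InventoryItem_Base is a base actor for inventory items, holding identity and type data alongside a Body static mesh.
; InitializeSpawnData stores the item's ID and SN.
; InitializeInventoryItemBaseData stores item type, name and damage type (in a variable spelled DamgeType) and sets the mesh on Body.
; The event graph and construction script add no logic of their own.
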(event EventBeginPlay
  (|CallParentFunction) ; This node is disabled and will not be called.\nDrag off pins to build functionality.
)

(event Collision|EventActorBeginOverlap
  (params (OtherActor :type Actor%20Object%20Reference))
  (|CallParentFunction OtherActor) ; This node is disabled and will not be called.\nDrag off pins to build functionality.
)

(event EventTick
  (params (DeltaSeconds :type Float%20%28single-precision%29))
  (|CallParentFunction DeltaSeconds) ; This node is disabled and will not be called.\nDrag off pins to build functionality.
)

(fn ConstructionScript
  (|CallParentFunction))

(fn InitializeSpawnData
  (params (ID :type Name) (SN :type String))
  (Variables|Default|SetID ID)
  (Variables|Default|SetSN SN))

(fn InitializeInventoryItemBaseData
  (params (ItemType :type E_ItemType%20Enum :default "NewEnumerator0") (ItemName :type Text) (StaticMesh :type Static%20Mesh%20Object%20Reference) (DamageType :type E_DamageType%20Enum :default "NewEnumerator0"))
  (Utilities|FlowControl|Sequence
    (:then_0
      (Variables|Default|SetItemType ItemType))
    (:then_1
      (Variables|Default|SetItemName ItemName))
    (:then_2
      (Components|StaticMesh|SetStaticMesh (Variables|Default|GetBody) StaticMesh))
    (:then_3
      (Variables|Default|SetDamgeType DamageType))))