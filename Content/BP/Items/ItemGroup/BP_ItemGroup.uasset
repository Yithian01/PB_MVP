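; BP_ItemGroup is an item group actor that generates random transforms around its own location.
; GetRandomTransforms loops over a requested Number, offsetting the actor's location by randomly scaled unit vectors with Z zeroed to keep points at the actor's height.
; Each transform has zero rotation and unit scale, and the function returns them as an array.
; The event graph and construction script contain no logic, and the file itself spawns nothing.
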(event EventBeginPlay)

(event Collision|EventActorBeginOverlap
  (params (OtherActor :type Actor%20Object%20Reference)))

(event EventTick
  (params (DeltaSeconds :type Float%20%28single-precision%29)))

(fn ConstructionScript)

(fn GetRandomTransforms
  (params (Number :type Integer))
  (bind _returnvalue (Math|Random|RandomFloatinRange 1e+02 2e+02))
  (bind _returnvalue_2 (Math|Random|RandomUnitVector))
  (bind _returnvalue_3 (* _returnvalue_2 _returnvalue))
  (for _index (range 0 Number)
    (Utilities|Array|Add (LocalVariables|GetReturnTransform) (Math|Transform|MakeTransform (+ (Transformation|GetActorLocation) (Math|Vector|MakeVector (.x _returnvalue_3) (.y _returnvalue_3) 0.0)))))
  (return (LocalVariables|GetReturnTransform)))