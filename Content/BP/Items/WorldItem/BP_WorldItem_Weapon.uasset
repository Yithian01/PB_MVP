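; BP_WorldItem_Weapon is a world item Blueprint for weapons, configured from a data table when it spawns.
; InitializeSpawnData calls the parent, then looks up the ID in DT_WorldItem_WeaponData and passes type, name, UI prefix, mesh and icon to the base initializer with outlining enabled.
; It also stores damage type and weight, sets the Body's world rotation and scale from the row, and uses weight as its mass override.
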(event EventBeginPlay
  (|CallParentFunction) ; This node is disabled and will not be called.\nDrag off pins to build functionality.
)

(event Collision|EventActorBeginOverlap
  (params (OtherActor :type Actor%20Object%20Reference))
  (|CallParentFunction OtherActor) ; This node is disabled and will not be called.\nDrag off pins to build functionality.
)

(event EventTick
  (params (DeltaSeconds :type Float%20%28single-precision%29))
  (|CallParentFunction DeltaSeconds) ; This node is disabled and will not be called.\nDrag off pins to build functionality.
)

(fn ConstructionScript
  (|CallParentFunction))

(fn InitializeSpawnData
  (params (ID :type Name :default "None") (SN :type String))
  (|CallParentFunction ID SN)
  (bind _returnvalue (Utilities|GetDataTableRow "/Game/BP/Datas/Datatable/Item/DT_WorldItem_WeaponData.DT_WorldItem_WeaponData" (Variables|Default|GetID))
    (:then
      (CallFunction|InitializeWorldItemBaseData (.itemtype _returnvalue) (.itemname _returnvalue) (.uiprefix _returnvalue) (.staticmesh _returnvalue) (.icon _returnvalue) true)
      (Variables|Default|SetDamageType (.damagetype _returnvalue))
      (Variables|Default|SetWight (.weight _returnvalue))
      (Transformation|SetWorldRotation (Variables|Default|GetBody) (.rotationoffset _returnvalue) false false)
      (Transformation|SetWorldScale3D (Variables|Default|GetBody) (.scaleoffset _returnvalue))
      (Class|PrimitiveComponent|SetMassOverrideinKg (Variables|Default|GetBody) "None" (Variables|Default|GetWight) true))))