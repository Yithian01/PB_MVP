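; Lobby game mode that names joining players, relays timestamped chat and starts the match with seamless travel to Step1.
; TryGameStart requires that at most one player is unready, then sets a start timer and a looping one-second timer.
; CalcuateLodingTime writes remaining countdown time to the lobby GameState.
; GameStart issues ServerTravel and notifies the GameState, which also receives chat messages formatted by MakeMessage.
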(event Custom|GameStart
  ;[0.15 0.15 0.15 0.5] GameStart
  (Development|ExecuteConsoleCommand (Utilities|String|ToString(Text) (Utilities|Text|FormatText "ServerTravel Step1")) (Game|GetPlayerController 0))
  (bind _asbp_lobby_game_state (Utilities|Casting|CastToBP_LobbyGameState (Game|GetGameState)))
  (Default|S2MEnterGameWorld _asbp_lobby_game_state)
  (Utilities|Time|ClearandInvalidateTimerbyHandle (Variables|Default|GetGameLodingHandler)))

(event Custom|TryGameStart
  (bind _readystate (CallFunction|IsPlayersReady))
  ;[0.15 0.15 0.15 0.5] Try GameStart
  (if _readystate
    (Variables|Default|SetbIsGameStartCountDown (and _readystate (not (Variables|Default|GetbIsGameStartCountDown))))
    (bind _output_get (Variables|Default|SetStartGameTime (+ (Utilities|Time|GetGameTimeinSeconds) (Variables|Default|GetStartLodingTime))))
    (Utilities|Time|SetTimerbyEvent (EventDispatchers|CreateEvent :!event Custom|GameStart) _output_get)
    (bind _returnvalue (Utilities|Time|SetTimerbyEvent (EventDispatchers|CreateEvent :!event CalcuateLodingTime) 1.0 true))
    (Variables|Default|SetGameLodingHandler _returnvalue)))

(event EventPostLogin
  (params (NewPlayer :type Player%20Controller%20Object%20Reference))
  ;[0.15 0.15 0.15 0.5] Login
  (bind _asbp_lobby_player_state (Utilities|Casting|CastToBP_LobbyPlayerState (Variables|/Script/Engine.Controller|GetPlayerState NewPlayer)))
  (bind _returnvalue (Class|GameModeBase|GetNumPlayers))
  (Variables|/Game/BP/Lobby/BP_LobbyPlayerState.BP_LobbyPlayerState_C|SetNickname _asbp_lobby_player_state (Utilities|Text|FormatText "Player_{0}" _returnvalue)))

(event EventBeginPlay
  ;[0.15 0.15 0.15 0.5] Seamless Travel
  (Variables|Default|SetbUseSeamlessTravel true))

(fn ConstructionScript)

(fn IsPlayersReady
  (for _array_element (Variables|/Script/Engine.GameStateBase|GetPlayerArray (Game|GetGameState))
    (bind _asbp_lobby_player_state (Utilities|Casting|CastToBP_LobbyPlayerState _array_element))
    (if (not (Variables|/Game/BP/Lobby/BP_LobbyPlayerState.BP_LobbyPlayerState_C|GetbIsReady _asbp_lobby_player_state))
      (bind _result (Math|Integer|IncrementInt (LocalVariables|GetLocalNotReadyCount))
        (:%20%20
          (if (>= _result 2)
            (return false))))))
  (return true))

(fn CalcuateLodingTime
  (bind _returnvalue (Utilities|Time|GetGameTimeinSeconds))
  (bind _startgametime (Variables|Default|GetStartGameTime))
  (bind _returnvalue_2 (- _startgametime _returnvalue))
  (bind _asbp_lobby_game_state (Utilities|Casting|CastToBP_LobbyGameState (Game|GetGameState)))
  (if (not (<= _returnvalue_2 0.0))
    (Variables|/Game/BP/Lobby/BP_LobbyGameState.BP_LobbyGameState_C|SetCurrentLodingTime _asbp_lobby_game_state _returnvalue_2)))

(fn MakeMessage
  (params (InMessage :type Text) (InPlayerState :type Player%20State%20Object%20Reference))
  (bind _asbp_lobby_player_state (Utilities|Casting|CastToBP_LobbyPlayerState InPlayerState))
  (LocalVariables|SetLocalSendPlayerState _asbp_lobby_player_state)
  (bind _asbp_lobby_game_state (Utilities|Casting|CastToBP_LobbyGameState (Game|GetGameState)))
  (Default|S2MUpdateChating _asbp_lobby_game_state (Utilities|Text|FormatText "{Nickname} {Time} : {Message}" (Variables|/Game/BP/Lobby/BP_LobbyPlayerState.BP_LobbyPlayerState_C|GetNickname _asbp_lobby_player_state) (Class|KismetTextLibrary|AsTimespanTimespan (TimeOfDay|GetTimeOfDay (Math|DateTime|Now) :!class /Script/Engine.KismetMathLibrary)) InMessage) (LocalVariables|GetLocalSendPlayerState)))