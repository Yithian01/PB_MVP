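; BP_LobbyGameState is the lobby game state that relays shared lobby events to the local player's BP_LobbyHud.
; S2M events, named as server-to-multicast RPCs, tell the HUD to start the game-world loading display or add a chat message with its sender's player state.
; CurrentLodingTime uses an OnRep handler to push the replicated loading time to the HUD.
; Each path casts player controller 0's HUD and does nothing if that fails.
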(event Custom|S2M_EnterGameWorld
  (bind _asbp_lobby_hud (Utilities|Casting|CastToBP_LobbyHud (HUD|GetHUD (Game|GetPlayerController 0))))
  (Default|EnterGameLoadingssd _asbp_lobby_hud))

(event Custom|S2M_UpdateChating
  (params (InMessage :type Text) (InPlayerState :type BP%20Lobby%20Player%20State%20Object%20Reference))
  (bind _asbp_lobby_hud (Utilities|Casting|CastToBP_LobbyHud (HUD|GetHUD (Game|GetPlayerController 0))))
  (Default|UpdateChating _asbp_lobby_hud InMessage InPlayerState))

(fn ConstructionScript)

(fn OnRepCurrentLodingTime
  (bind _asbp_lobby_hud (Utilities|Casting|CastToBP_LobbyHud (HUD|GetHUD (Game|GetPlayerController 0))))
  (Default|UpdateLodingTime _asbp_lobby_hud (Variables|Default|GetCurrentLodingTime)))