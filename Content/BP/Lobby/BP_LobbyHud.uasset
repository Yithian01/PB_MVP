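; BP_LobbyHud is the lobby HUD that creates and owns the WBP_Lobby widget for the local lobby player controller.
; On BeginPlay it caches the controller, passes it into the widget and adds that widget to the viewport.
; RefreshUI, also triggered by S2M_UpdateLobbyUI, retries every 0.2 seconds until the widget is valid.
; Helper functions forward loading time, the loading popup and chat messages to the widget.
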(event Custom|RefreshUI
  (Utilities|IsValid (Variables|Default|GetLobbyUIRef) :!label _label
    (:Is%20Valid
      (Default|RefreshUI (Variables|Default|GetLobbyUIRef)))
    (:Is%20Not%20Valid
      (Utilities|FlowControl|Delay 0.2)
      (goto _label))))

(event EventBeginPlay
  (Utilities|FlowControl|Sequence
    (:then_0
      (bind _asbp_lobby_player_controller (Utilities|Casting|CastToBP_LobbyPlayerController (Game|GetPlayerController 0)))
      (Variables|Default|SetLobbyPlayerControllerRef _asbp_lobby_player_controller))
    (:then_1
      (Utilities|IsValid (Variables|Default|GetLobbyPlayerControllerRef)
        (:Is%20Valid
          (bind _returnvalue (UserInterface|CreateWidget "/Widget/Lobby/WBP_Lobby.WBP_Lobby_C" 0 (Variables|Default|GetLobbyPlayerControllerRef)))
          (bind _output_get (Variables|Default|SetLobbyUIRef _returnvalue))
          (UserInterface|Viewport|AddtoViewport _output_get 0))))))

(event Custom|S2M_UpdateLobbyUI
  (CallFunction|RefreshUI))

(fn ConstructionScript)

(fn UpdateLodingTime
  (params (InTime :type Float%20%28double-precision%29))
  (Default|UpdateLogindTime (Variables|Default|GetLobbyUIRef) (Math|Float|Truncate InTime)))

(fn EnterGameLoadingssd
  (Default|LodingPopup (Variables|Default|GetLobbyUIRef)))

(fn UpdateChating
  (params (InMessage :type Text) (InPlayerState :type BP%20Lobby%20Player%20State%20Object%20Reference))
  (Default|UpdateChating (Variables|Default|GetLobbyUIRef) InMessage InPlayerState))