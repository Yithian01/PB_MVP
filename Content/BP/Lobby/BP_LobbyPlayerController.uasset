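; Lobby player controller that sets UI-only input with a visible cursor and relays game-start and lobby UI refresh requests.
; CallGameStart fires the client-to-server start event, which calls GameStart on BP_LobbyGameMode.
; S2M_UpdateLobbyUI tells the BP_LobbyHud to refresh its UI, with the C2S and S2M prefixes marking the intended RPC direction.
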(event EventBeginPlay
  (Utilities|FlowControl|Sequence
    (:then_0
      (Input|SetInputModeUIOnly self 0 "DoNotLock" false)
      (Variables|Default|SetbShowMouseCursor true))))

(event Custom|S2M_UpdateLobbyUI
  (bind _asbp_lobby_hud (Utilities|Casting|CastToBP_LobbyHud (HUD|GetHUD)))
  (Default|RefreshUI _asbp_lobby_hud))

(event Custom|C2S_GameStart
  (bind _asbp_lobby_game_mode (Utilities|Casting|CastToBP_LobbyGameMode (Game|GetGameMode)))
  (Default|GameStart _asbp_lobby_game_mode))

(event Custom|CallGameStart
  (CallFunction|C2SGameStart))

(fn ConstructionScript)