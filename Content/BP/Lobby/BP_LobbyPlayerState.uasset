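; Lobby player state that tracks a player's nickname and ready flag and keeps the lobby UI in sync.
; BeginPlay, destruction, nickname OnRep and ready toggles all call CallUpdateUI, which refreshes the UI through the local BP_LobbyPlayerController.
; Server-to-multicast and server-to-client events, as their prefixes indicate, flip the ready flag and send a kicked player to the Title level.
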(event Custom|OnDestroyed_Event
  (params (DestroyedActor :type Actor%20Object%20Reference))
  (CallFunction|CallUpdateUI))

(event EventBeginPlay
  (Development|PrintString "Hello" true true "(R=0.000000,G=0.660000,B=1.000000,A=1.000000)" 999.0)
  (CallFunction|CallUpdateUI)
  (Game|AssignOnDestroyed (delegate Custom|OnDestroyed_Event)))

(event Custom|S2C_HandleKickPlayer
  (Game|OpenLevel(byObjectReference) "/Game/Maps/Title.Title"))

(event Custom|S2M_HandleReadyButton
  (Variables|Default|SetbIsReady (not (Variables|Default|GetbIsReady)))
  (CallFunction|CallUpdateUI))

(fn ConstructionScript)

(fn OnRepNickname
  (Development|PrintString (Utilities|String|ToString(Text) (Utilities|Text|FormatText "PS = {0} 의 Nickname 변경됨" 0)) true true "(R=0.000000,G=0.660000,B=1.000000,A=1.000000)" 999.0)
  (CallFunction|CallUpdateUI))

(fn CallUpdateUI
  (bind _returnvalue (Game|GetPlayerController 0))
  (Utilities|IsValid _returnvalue
    (:Is%20Valid
      (bind _asbp_lobby_player_controller (Utilities|Casting|CastToBP_LobbyPlayerController _returnvalue))
      (Default|UpdateLobbyUI _asbp_lobby_player_controller))))