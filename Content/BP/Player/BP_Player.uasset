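; Player character handling movement, quick-slot inventory with hand-socketed items, montage attacks, and grabbing/throwing of break actors.
; A looping timer sphere-traces nearby items with line-of-sight checks, then a camera trace picks the outlined target for pickup or grab.
; BP_GameMode spawns and destroys items, while a DataTable resolves pose transitions.
; Thrown break-actor hits apply stun damage that can trigger ragdoll until an HP-recovery timeline finishes.
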(event OnComponentHit(CapsuleComponent)
  (params (HitComponent :type Primitive%20Component%20Object%20Reference) (OtherActor :type Actor%20Object%20Reference) (OtherComp :type Primitive%20Component%20Object%20Reference) (NormalImpulse :type Vector :default "0, 0, 0") (Hit :type Hit%20Result%20Structure%20%28by%20ref%29))
  (bind _asbp_break_actor_base (Utilities|Casting|CastToBP_BreakActor_Base OtherActor))
  (if (Default|IsThrow _asbp_break_actor_base)
    (if (Variables|Grab|GetbIsDamageEnable)
      (Interaction|DamgeEnable false)
      (Utilities|Time|SetTimerbyEvent (EventDispatchers|CreateEvent :!event Custom|EnableDamage) 0.36)
      (bind _bisstun (Default|TakeDamage (Variables|Default|GetBPC_StatAttribute) (Variables|/Game/BP/BreakActor/BP_BreakActor_Base.BP_BreakActor_Base_C|GetStunValue _asbp_break_actor_base)))
      (if _bisstun
        (Regdoll|StartRegdoll)
        (bind _alpha (Timeline|TL_RecoveryHp PlayFromStart)
          (:Update
            (Default|RecoverHp (Variables|Default|GetBPC_StatAttribute) (Math|Float|Lerp 0.0 (Variables|/Game/BP/Components/StatAttributeComponent/BPC_StunSystem.BPC_StunSystem_C|GetMaxHp (Variables|Default|GetBPC_StatAttribute)) _alpha)))
          (:Finished
            (Regdoll|RecoveryRegdoll)))))))

(event Custom|SearchWorldItem
  ;[0.15 0.15 0.15 0.5] BeginPlay
  (WorldItem|UpdateVicinityList)
  (WorldItem|UpdateTargetingItem))

(event Custom|OnEndGrab
  (Variables|Grab|SetbIsGrabedItem false)
  (Utilities|IsValid (Variables|Item|GetEquippedItem)
    (:Is%20Valid
      (Utilities|FlowControl|Delay 1.0)
      (Rendering|SetVisibility (Variables|/Game/BP/Items/InventoryItem/BP_InventoryItem_Base.BP_InventoryItem_Base_C|GetBody (Variables|Item|GetEquippedItem)) true false))))

(event Custom|OnStartGrab
  (Variables|Grab|SetbIsGrabedItem true)
  (Utilities|IsValid (Variables|Item|GetEquippedItem)
    (:Is%20Valid
      (Rendering|SetVisibility (Variables|/Game/BP/Items/InventoryItem/BP_InventoryItem_Base.BP_InventoryItem_Base_C|GetBody (Variables|Item|GetEquippedItem)) false false))))

(event Custom|EnableDamage
  (Interaction|DamgeEnable true))

(event EventBeginPlay
  ;[0.15 0.15 0.15 0.5] BeginPlay
  (Utilities|FlowControl|Sequence
    (:then_0
      (bind _asbp_game_mode (Utilities|Casting|CastToBP_GameMode (Game|GetGameMode)))
      (Variables|Ref|SetGameModeRef _asbp_game_mode))
    (:then_1
      (Variables|Regdoll|SetOriginTransform (Transformation|GetRelativeTransform (Variables|Character|GetMesh))))
    (:then_2
      (Utilities|Time|SetTimerbyEvent (delegate Custom|SearchWorldItem) 0.05 true))))

(event EventTick
  (params (DeltaSeconds :type Float%20%28single-precision%29))
  ;[0.15 0.15 0.15 0.5] Debug
  (Development|PrintString (Utilities|String|ToString(Text) (Utilities|Text|FormatText "Debug to BP_Player 
Pose State : {0} 
현재 무기 타입 : {1} 
현재 타겟 아이템: {2}" (Utilities|String|EnumtoString (Variables|Pose|GetCurrentPose)) (Utilities|String|EnumtoString (Attack|GetWeaponDamageType)) (Variables|Item|GetLast%20TargetItem))) true true "(R=0.000000,G=0.660000,B=1.000000,A=1.000000)" 0.0))

(fn ConstructionScript)

(fn Move
  (params (bIsForward :type Boolean) (AxisValue :type Float%20%28double-precision%29))
  (Pawn|Input|AddMovementInput (Math|Vector|SelectVector (Transformation|GetActorForwardVector) (Transformation|GetActorRightVector) bIsForward) AxisValue false))

(fn Look
  (params (bIsLookUp :type Boolean) (AxisValue :type Float%20%28double-precision%29))
  (if bIsLookUp
    (Pawn|Input|AddControllerPitchInput AxisValue)
    (else
      (Pawn|Input|AddControllerYawInput AxisValue))))

(fn DropItem
  (bind _returnvalue (Transformation|GetActorTransform))
  (Utilities|IsValid (Variables|Item|GetEquippedItem)
    (:Is%20Valid
      (if (not (Variables|Grab|GetbIsGrabedItem))
        (Utilities|FlowControl|Sequence
          (:then_0
            (Default|GenerateInventorytoWorldItem (Variables|Ref|GetGameModeRef) (Math|Transform|MakeTransform (Transformation|GetWorldLocation (Variables|Default|GetCamera)) (.rotation _returnvalue) (.scale _returnvalue)) (Variables|/Game/BP/Items/BP_ItemBase.BP_ItemBase_C|GetID (Variables|Item|GetEquippedItem)) (* (Math|Vector|GetForwardVector (Variables|Default|GetCamera)) (Variables|Item|GetDropItemForce))))
          (:then_1
            (Default|RemoveItem (Variables|Default|GetBPC_Inventory)))
          (:then_2
            (Default|DestoryInventoryItem (Variables|Ref|GetGameModeRef) (Variables|Item|GetEquippedItem))))))))

(fn SelectQuickSlot
  (params (Index :type Integer))
  (if (not (Variables|Grab|GetbIsGrabedItem))
    (bind _currentid (Default|SelectQuickSlot (Variables|Default|GetBPC_Inventory) Index))
    (Utilities|FlowControl|Sequence
      (:then_0
        (Utilities|IsValid (Variables|Item|GetEquippedItem)
          (:Is%20Valid
            (Default|DestoryInventoryItem (Variables|Ref|GetGameModeRef) (Variables|Item|GetEquippedItem)))))
      (:then_1
        (if (!= _currentid "")
          (bind _spawnitem (Default|GenerateInventoryItemWeapon (Variables|Ref|GetGameModeRef) _currentid))
          (bind _output_get (Variables|Item|SetEquippedItem _spawnitem))
          (Transformation|AttachComponentToComponent _output_get (Variables|Character|GetMesh) "HandGrip_R" "SnapToTarget" "SnapToTarget" "SnapToTarget" true))))))

(fn GetVicinityItems
  (bind _returnvalue (Transformation|GetActorLocation))
  (bind (_outhits _returnvalue_2) (Collision|MultiSphereTraceForObjects _returnvalue _returnvalue 2.2e+02 (Utilities|Array|MakeArray "ObjectTypeQuery7" "ObjectTypeQuery9") false 0 "None"))
  (if _returnvalue_2
    (bind _arrayelement (Utilities|Array|ReverseforEachLoop _outhits)
      (:LoopBody
        (bind _outhit (Collision|LineTraceByChannel (Transformation|GetActorLocation) (+ (* (.impactnormal _arrayelement) -2e+01) (Transformation|GetActorLocation (.hitactor _arrayelement))) "TraceTypeQuery1" false 0 "None" true "(R=0.170243,G=1.000000,B=0.454102,A=1.000000)"))
        (if true
          (if (== (.hitactor _arrayelement) (.hitactor _outhit))
            (Utilities|Set|Add (LocalVariables|GetCurrentItems) (.hitactor _outhit)))))
      (:Completed
        (return (LocalVariables|GetCurrentItems))))))

(fn UpdateVicinityList
  (Utilities|FlowControl|Sequence
    (:then_0
      (LocalVariables|SetPrevVicinityList (Variables|Item|GetCurrentVicinityList))
      (bind _output_get (LocalVariables|SetNewVicinityList (WorldItem|GetVicinityItems)))
      (if (== (Utilities|Set|Length _output_get) (Utilities|Set|Length (LocalVariables|GetPrevVicinityList)))
        (bind _valuepin (Utilities|Set|ForEachLoop(Set) (LocalVariables|GetNewVicinityList) :!label _label)
          (:then
            (if (not (Utilities|Set|Contains (LocalVariables|GetPrevVicinityList) _valuepin))
              (LocalVariables|SetNeedUpdate true)
              (goto _label BreakPin))))
        (else
          (LocalVariables|SetNeedUpdate true))))
    (:then_1
      (if (LocalVariables|GetNeedUpdate)
        (Utilities|Set|Clear (Variables|Item|GetCurrentVicinityList))
        (bind _valuepin_2 (Utilities|Set|ForEachLoop(Set) (LocalVariables|GetNewVicinityList))
          (:then
            (bind _asbp_world_item_base (Utilities|Casting|CastToBP_WorldItem_Base _valuepin_2))
            (Utilities|Set|Add (Variables|Item|GetCurrentVicinityList) _asbp_world_item_base)))))))

(fn UpdateTargetingItem
  (bind _camera (Variables|Default|GetCamera))
  (bind _returnvalue (Transformation|GetWorldLocation _camera))
  (if (Utilities|Set|IsEmpty (Variables|Item|GetCurrentVicinityList))
    (Utilities|IsValid (Variables|Item|GetLast%20TargetItem)
      (:Is%20Valid
        (Default|EnableOutline (Variables|Item|GetLast%20TargetItem) false)
        (Variables|Item|SetLast%20TargetItem 0)))
    (else
      (bind (_outhit _returnvalue_2) (Collision|LineTraceByChannel _returnvalue (+ _returnvalue (* (Math|Vector|GetForwardVector _camera) (Variables|Item|GetPickUpRange))) "TraceTypeQuery1" false 0 "None" true "(R=0.815871,G=0.148143,B=1.000000,A=1.000000)"))
      (if _returnvalue_2
        (bind _valuepin (Utilities|Set|ForEachLoop(Set) (Variables|Item|GetCurrentVicinityList))
          (:then
            (Default|EnableOutline _valuepin false)
            (if (< (Math|Vector|Distance(Vector) (Transformation|GetActorLocation _valuepin) (Transformation|GetActorLocation (.HitActor (Collision|BreakHitResult _outhit)))) (LocalVariables|GetClosestDistance))
              (LocalVariables|SetClosestDistance (Math|Vector|Distance(Vector) (Transformation|GetActorLocation _valuepin) (Transformation|GetActorLocation (.HitActor (Collision|BreakHitResult _outhit)))))
              (LocalVariables|SetCurrentTargetItem _valuepin)))
          (:CompletedPin
            (if (< (LocalVariables|GetClosestDistance) 1e+02)
              (Default|EnableOutline (LocalVariables|GetCurrentTargetItem) true)
              (Variables|Item|SetLast%20TargetItem (LocalVariables|GetCurrentTargetItem))
              (else
                (LocalVariables|SetCurrentTargetItem 0)))))))))

(fn OldPickUpItem
  (bind _camera (Variables|Default|GetCamera))
  (bind _returnvalue (Transformation|GetWorldLocation _camera))
  (bind (_outhit _returnvalue_2) (Collision|LineTraceForObjects _returnvalue (+ _returnvalue (* (.WorldDirection (Class|GameplayStatics|DeprojectScreentoWorld (Game|GetPlayerController 0) (/ (Viewport|GetViewportSize) "(X=2.000000,Y=2.000000)"))) (Variables|Item|GetPickUpRange))) (Utilities|Array|MakeArray "ObjectTypeQuery7") false 0 "ForDuration"))
  (if _returnvalue_2
    (bind _asbp_world_item_base (Utilities|Casting|CastToBP_WorldItem_Base (.HitActor (Collision|BreakHitResult _outhit))))
    (bind _output_get (LocalVariables|SetCurrentWorldItem _asbp_world_item_base))
    (bind _success (Default|AddItem (Variables|Default|GetBPC_Inventory) (Variables|/Game/BP/Items/BP_ItemBase.BP_ItemBase_C|GetItemType _output_get) (Variables|/Game/BP/Items/BP_ItemBase.BP_ItemBase_C|GetID _output_get) 1 (Variables|/Game/BP/Items/WorldItem/BP_WorldItem_Base.BP_WorldItem_Base_C|GetIcon _output_get)))
    (if _success
      (WorldItem|SelectQuickSlot (Variables|/Game/BP/Components/InventoryComponent/BPC_Inventory.BPC_Inventory_C|GetCurrentSelectIndex (Variables|Default|GetBPC_Inventory)))
      (Default|DestoryWorldItem (Variables|Ref|GetGameModeRef) (LocalVariables|GetCurrentWorldItem)))))

(fn PickUpItem
  (bind _last_targetitem (Variables|Item|GetLast%20TargetItem))
  (Utilities|IsValid (Variables|Item|GetLast%20TargetItem)
    (:Is%20Valid
      (Utilities|Casting|CastToBP_BreakActor_Base (Variables|Item|GetLast%20TargetItem)
        (:CastFailed
          (bind _success (Default|AddItem (Variables|Default|GetBPC_Inventory) (Variables|/Game/BP/Items/BP_ItemBase.BP_ItemBase_C|GetItemType _last_targetitem) (Variables|/Game/BP/Items/BP_ItemBase.BP_ItemBase_C|GetID _last_targetitem) 1 (Variables|/Game/BP/Items/WorldItem/BP_WorldItem_Base.BP_WorldItem_Base_C|GetIcon _last_targetitem)))
          (if _success
            (WorldItem|SelectQuickSlot (Variables|/Game/BP/Components/InventoryComponent/BPC_Inventory.BPC_Inventory_C|GetCurrentSelectIndex (Variables|Default|GetBPC_Inventory)))
            (Default|DestoryWorldItem (Variables|Ref|GetGameModeRef) (Variables|Item|GetLast%20TargetItem))))))))

(fn UpdatePoseState
  (params (NewState :type E_PoseState%20Enum :default "NewEnumerator0"))
  (Variables|Pose|SetCurrentPose NewState))

(fn TryGetPoseTransition
  (params (TargetPose :type E_PoseState%20Enum :default "NewEnumerator0"))
  (bind _returnvalue (Utilities|GetDataTableRow "/Game/BP/Datas/Datatable/Player/DT_PoseTransitionRule.DT_PoseTransitionRule" (Utilities|String|StringToName (Utilities|String|Append (Utilities|String|EnumtoString TargetPose) "_" (Utilities|String|EnumtoString (Variables|Pose|GetCurrentPose)))))
    (:then
      (return (.topose _returnvalue)))))

(fn GetWeaponDamageType
  (bind _equippeditem (Variables|Item|GetEquippedItem))
  (Utilities|IsValid _equippeditem
    (:Is%20Valid
      (return (Variables|/Game/BP/Items/InventoryItem/BP_InventoryItem_Base.BP_InventoryItem_Base_C|GetDamgeType _equippeditem)))
    (:Is%20Not%20Valid
      (return "NewEnumerator0"))))

(fn EnableAttackState
  (Variables|Attack|SetEnableAttack true))

(fn Attack
  (if (and (Variables|Attack|GetEnableAttack) (not (Variables|Grab|GetbIsGrabedItem)))
    (Variables|Attack|SetEnableAttack false)
    (bind _returnvalue (Animation|PlayAnimMontage "/Game/BP/Player/Animation/Attack/AM_Attack.AM_Attack" 1.0 "None"))
    (Utilities|Time|SetTimerbyEvent (EventDispatchers|CreateEvent :!event EnableAttackState) _returnvalue)))

(fn DamgeEnable
  (params (Enable :type Boolean))
  (Variables|Grab|SetbIsDamageEnable Enable))

(fn ToggleGrab
  (if (Default|IsGrab (Variables|Default|GetBPC_Grabber))
    (bind _returnitem (Default|ReleaseGrab (Variables|Default|GetBPC_Grabber)))
    (bind _output_get (LocalVariables|SetRelaseItem _returnitem))
    (Transformation|DetachFromActor _output_get "KeepWorld" "KeepWorld" "KeepWorld")
    (Transformation|SetWorldLocation (Variables|/Game/BP/Items/BP_ItemBase.BP_ItemBase_C|GetDefaultSceneRoot (LocalVariables|GetRelaseItem)) (+ (Transformation|GetWorldLocation (Variables|/Game/BP/Items/BP_ItemBase.BP_ItemBase_C|GetDefaultSceneRoot (LocalVariables|GetRelaseItem))) (* (Math|Vector|GetForwardVector (Variables|Default|GetCamera)) 5e+01)) false false)
    (Default|OnReleaseGrab (LocalVariables|GetRelaseItem))
    (Default|EnableOutline (LocalVariables|GetRelaseItem) false)
    (Physics|AddImpulse (Variables|/Game/BP/Items/WorldItem/BP_WorldItem_Base.BP_WorldItem_Base_C|GetBody (LocalVariables|GetRelaseItem)) (* (Math|Vector|GetForwardVector (Variables|Default|GetCamera)) (Variables|Item|GetThrowImpulse)) "None" false)
    (CallFunction|OnEndGrab)
    (else
      (Utilities|IsValid (Variables|Item|GetLast%20TargetItem)
        (:Is%20Valid
          (bind _asbp_break_actor_base (Utilities|Casting|CastToBP_BreakActor_Base (Variables|Item|GetLast%20TargetItem)))
          (bind _output_get_2 (LocalVariables|SetCurrentGrabItem _asbp_break_actor_base))
          (bind _newparam (Default|CanGrab (Variables|/Game/BP/BreakActor/BP_BreakActor_Base.BP_BreakActor_Base_C|GetBPC_Grabbable _output_get_2)))
          (if _newparam
            (bind _bissuccess (Default|TryGrab (Variables|Default|GetBPC_Grabber) _output_get_2))
            (if _bissuccess
              (Default|OnGrabbed (LocalVariables|GetCurrentGrabItem))
              (Transformation|AttachComponentToComponent (LocalVariables|GetCurrentGrabItem) (Variables|Character|GetMesh) "GrabSocket" "SnapToTarget" "SnapToTarget" "SnapToTarget" true)
              (CallFunction|OnStartGrab))))))))

(fn StartRegdoll
  (Utilities|FlowControl|Sequence
    (:then_0
      (Variables|Regdoll|SetbIsRegdoll true)
      (Pawn|Components|CharacterMovement|DisableMovement (Variables|Character|GetCharacterMovement)))
    (:then_1
      (Collision|SetCollisionEnabled (Variables|Collision|GetCapsuleComponent) "NoCollision")
      (Collision|SetCollisionEnabled (Variables|Character|GetMesh) "QueryAndPhysics"))
    (:then_2
      (Physics|SetSimulatePhysics (Variables|Character|GetMesh) true))))

(fn RecoveryRegdoll
  (Utilities|FlowControl|Sequence
    (:then_0
      (Physics|SetSimulatePhysics (Variables|Character|GetMesh) false))
    (:then_1
      (Transformation|SetActorLocation (Transformation|GetWorldLocation (Variables|Character|GetMesh)) false false))
    (:then_2
      (Transformation|SetRelativeRotation (Variables|Character|GetMesh) (Math|Rotator|MakeRotator 0.0 0.0 (.yaw (Transformation|GetActorRotation))) false false)
      (Transformation|SetRelativeTransform (Variables|Character|GetMesh) (Variables|Regdoll|GetOriginTransform) false false))
    (:then_3
      (Collision|SetCollisionEnabled (Variables|Collision|GetCapsuleComponent) "QueryAndPhysics")
      (Collision|SetCollisionEnabled (Variables|Character|GetMesh) "NoCollision"))
    (:then_4
      (Pawn|Components|CharacterMovement|SetMovementMode (Variables|Character|GetCharacterMovement) "MOVE_Walking" 0)
      (Variables|Regdoll|SetbIsRegdoll false))))