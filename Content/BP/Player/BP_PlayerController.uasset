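; Player controller that forwards the player's input to BP_Player and manages cursor and input mode for gameplay and the game's end.
; On BeginPlay it locks input to game-only, caches the player character and game mode, and binds EndGame to the game mode's result event, which restores the cursor and UI input.
; Axis and action events relay movement, look, jump, quick slots, item pickup and drop, crouch, grab and attack to the character.
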(event Custom|EndGame
  (Variables|Default|SetbShowMouseCursor true)
  (Input|SetInputModeGameandUI self 0 "DoNotLock" true true))

(event EventBeginPlay
  (Utilities|FlowControl|Sequence
    (:then_0
      (Variables|Default|SetbShowMouseCursor false)
      (Input|SetInputModeGameOnly self true))
    (:then_1
      (bind _asbp_player (Utilities|Casting|CastToBP_Player (Game|GetPlayerCharacter 0)))
      (Variables|Default|SetPlayerRef _asbp_player))
    (:then_2
      (bind _asbp_game_mode (Utilities|Casting|CastToBP_GameMode (Game|GetGameMode)))
      (bind _output_get (Variables|Default|SetGameModeRef _asbp_game_mode))
      (EventDispatchers|BindEventtoShowGameResult _output_get (delegate Custom|EndGame)))))

(event Input|ActionEvents|InputActionJumpping
  (params (Key :type Key%20Structure))
  ;[0.15 0.15 0.15 0.5] Jumpping
  (:Pressed
    (Character|Jump (Variables|Default|GetPlayerRef))))

(event Input|ActionEvents|InputActionPickUp
  (params (Key :type Key%20Structure))
  ;[0.15 0.15 0.15 0.5] PickUp Item
  (:Pressed
    (Default|PickUpItem (Variables|Default|GetPlayerRef))))

(event Input|ActionEvents|InputActionDropItem
  (params (Key :type Key%20Structure))
  ;[0.15 0.15 0.15 0.5] Drop Item
  (:Pressed
    (Default|DropItem (Variables|Default|GetPlayerRef))))

(event Input|ActionEvents|InputActionQuickSlot_1
  (params (Key :type Key%20Structure))
  ;[0.15 0.15 0.15 0.5] QuickSlot
  (:Pressed
    (Default|SelectQuickSlot (Variables|Default|GetPlayerRef))))

(event Input|ActionEvents|InputActionQuickSlot_2
  (params (Key :type Key%20Structure))
  ;[0.15 0.15 0.15 0.5] QuickSlot
  (:Pressed
    (Default|SelectQuickSlot (Variables|Default|GetPlayerRef) 1)))

(event Input|ActionEvents|InputActionQuickSlot_3
  (params (Key :type Key%20Structure))
  ;[0.15 0.15 0.15 0.5] QuickSlot
  (:Pressed
    (Default|SelectQuickSlot (Variables|Default|GetPlayerRef) 2)))

(event Input|ActionEvents|InputActionCrouch
  (params (Key :type Key%20Structure))
  ;[0.15 0.15 0.15 0.5] Pose State
  (:Pressed
    (bind _newparam (Default|TryGetPoseTransition (Variables|Default|GetPlayerRef) "NewEnumerator1"))
    (Default|UpdatePoseState (Variables|Default|GetPlayerRef) _newparam)))

(event Input|ActionEvents|InputActionAttack
  (params (Key :type Key%20Structure))
  (:Pressed
    (Default|Attack (Variables|Default|GetPlayerRef))))

(event Input|ActionEvents|InputActionGrab
  (params (Key :type Key%20Structure))
  ;[0.15 0.15 0.15 0.5] Pose State
  (:Pressed
    (Default|ToggleGrab (Variables|Default|GetPlayerRef))))

(event Input|AxisEvents|InputAxisMoveForward
  (params (AxisValue :type Float%20%28single-precision%29))
  ;[0.15 0.15 0.15 0.5] Move
  (Default|Move (Variables|Default|GetPlayerRef) true AxisValue))

(event Input|AxisEvents|InputAxisMoveRight
  (params (AxisValue :type Float%20%28single-precision%29))
  ;[0.15 0.15 0.15 0.5] Move
  (Default|Move (Variables|Default|GetPlayerRef) false AxisValue))

(event Input|AxisEvents|InputAxisLookUp
  (params (AxisValue :type Float%20%28single-precision%29))
  ;[0.15 0.15 0.15 0.5] Look
  (Default|Look (Variables|Default|GetPlayerRef) true AxisValue))

(event Input|AxisEvents|InputAxisLookTurn
  (params (AxisValue :type Float%20%28single-precision%29))
  ;[0.15 0.15 0.15 0.5] Look
  (Default|Look (Variables|Default|GetPlayerRef) false AxisValue))

(fn ConstructionScript)