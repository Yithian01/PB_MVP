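; Player controller for the title level that opens and closes a dashboard board UI.
; On BeginPlay it sets game-only input, caches the BP_Player reference and adds the default Enhanced Input mapping for the local player.
; The interaction action, while IsInDashBoard is set, lazily creates WBP_InBoard with UI-only input or re-shows it without changing input mode.
; CloseBoardUI collapses the widget and restores game-only input without the cursor.
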(event Input|EnhancedActionEvents|EnhancedInputActionIA_Interaction
  (params (ActionValue :type Boolean) (ElapsedSeconds :type Float%20%28double-precision%29) (TriggeredSeconds :type Float%20%28double-precision%29) (InputAction :type Input%20Action%20Object%20Reference :default "/Game/BP/Game/Input/Actions/IA_Interaction.IA_Interaction"))
  ;[0.15 0.15 0.15 0.5] Interaction DashBoard
  (:Started
    (if (Variables|Default|GetbIsInDashBoard)
      (Utilities|IsValid (Variables|Default|GetBoardUI_Ref)
        (:Is%20Valid
          (Widget|SetVisibility (Variables|Default|GetBoardUI_Ref) "Visible")
          (Variables|Default|SetbShowMouseCursor true))
        (:Is%20Not%20Valid
          (bind _returnvalue (UserInterface|CreateWidget "/Game/UI/Title/WBP_InBoard.WBP_InBoard_C"))
          (bind _output_get (Variables|Default|SetBoardUI_Ref _returnvalue))
          (UserInterface|Viewport|AddtoViewport _output_get 0)
          (Input|SetInputModeUIOnly self 0 "DoNotLock" true)
          (Variables|Default|SetbShowMouseCursor true))))))

(event EventBeginPlay
  ;[0.15 0.15 0.15 0.5] Initialize
  (Utilities|FlowControl|Sequence
    (:then_0
      (Variables|Default|SetbShowMouseCursor false)
      (Input|SetInputModeGameOnly self true))
    (:then_1
      (bind _asbp_player (Utilities|Casting|CastToBP_Player (Game|GetPlayerCharacter 0)))
      (Variables|Default|SetPlayerRef _asbp_player))
    (:then_2
      (if (Pawn|IsLocalPlayerController)
        (Input|AddMappingContext (PlayerController|LocalPlayerSubsystems|GetEnhancedInputLocalPlayerSubsystem) "/Game/BP/Game/Input/IMC_Default.IMC_Default" 0 "(bIgnoreAllPressedKeysUntilRelease=True,bForceImmediately=False,bNotifyUserSettings=False)")))))

(fn ConstructionScript)

(fn CloseBoardUI
  (Widget|SetVisibility (Variables|Default|GetBoardUI_Ref) "Collapsed")
  (Input|SetInputModeGameOnly self true)
  (Variables|Default|SetbShowMouseCursor false))