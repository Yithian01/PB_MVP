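; BP_DashBoard is a dashboard actor for the title area that detects when the player is within interaction range.
; Overlap events on its Box component cast the actor to BP_Player, then its controller to BP_PlayerController_Title, and set or clear that controller's IsInDashBoard flag.
; The same events show the Interaction component on entry and hide it on exit.
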(event OnComponentBeginOverlap(Box)
  (params (OverlappedComponent :type Primitive%20Component%20Object%20Reference) (OtherActor :type Actor%20Object%20Reference) (OtherComp :type Primitive%20Component%20Object%20Reference) (OtherBodyIndex :type Integer) (bFromSweep :type Boolean) (SweepResult :type Hit%20Result%20Structure%20%28by%20ref%29))
  (bind _asbp_player (Utilities|Casting|CastToBP_Player OtherActor))
  (bind _asbp_player_controller_title (Utilities|Casting|CastToBP_PlayerController_Title (Pawn|GetController _asbp_player)))
  (Variables|/Game/BP/Title/BP_PlayerController_Title.BP_PlayerController_Title_C|SetbIsInDashBoard _asbp_player_controller_title true)
  (Rendering|SetVisibility (Variables|Default|GetInteraction) true false))

(event OnComponentEndOverlap(Box)
  (params (OverlappedComponent :type Primitive%20Component%20Object%20Reference) (OtherActor :type Actor%20Object%20Reference) (OtherComp :type Primitive%20Component%20Object%20Reference) (OtherBodyIndex :type Integer))
  (bind _asbp_player (Utilities|Casting|CastToBP_Player OtherActor))
  (bind _asbp_player_controller_title (Utilities|Casting|CastToBP_PlayerController_Title (Pawn|GetController _asbp_player)))
  (Variables|/Game/BP/Title/BP_PlayerController_Title.BP_PlayerController_Title_C|SetbIsInDashBoard _asbp_player_controller_title false)
  (Rendering|SetVisibility (Variables|Default|GetInteraction) false false))

(fn ConstructionScript)