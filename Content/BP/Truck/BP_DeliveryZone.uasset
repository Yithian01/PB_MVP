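; Truck delivery zone actor that reports breakable objects entering or leaving its scoring volume and animates a wing hatch.
; On BeginPlay, a timeline lerps the left wing mesh's pitch from its starting value to a destination pitch, preserving roll and yaw.
; ScoreZone begin and end overlaps filter for BP_BreakActor_Base, then both fire the same OnUpdateScoreZone dispatcher with that actor, leaving score handling to listeners.
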(event OnComponentBeginOverlap(ScoreZone)
  (params (OverlappedComponent :type Primitive%20Component%20Object%20Reference) (OtherActor :type Actor%20Object%20Reference) (OtherComp :type Primitive%20Component%20Object%20Reference) (OtherBodyIndex :type Integer) (bFromSweep :type Boolean) (SweepResult :type Hit%20Result%20Structure%20%28by%20ref%29))
  (bind _asbp_break_actor_base (Utilities|Casting|CastToBP_BreakActor_Base OtherActor))
  (Default|CallOnUpdateScoreZone _asbp_break_actor_base))

(event OnComponentEndOverlap(ScoreZone)
  (params (OverlappedComponent :type Primitive%20Component%20Object%20Reference) (OtherActor :type Actor%20Object%20Reference) (OtherComp :type Primitive%20Component%20Object%20Reference) (OtherBodyIndex :type Integer))
  (bind _asbp_break_actor_base (Utilities|Casting|CastToBP_BreakActor_Base OtherActor))
  (Default|CallOnUpdateScoreZone _asbp_break_actor_base))

(event EventBeginPlay
  (CallFunction|HatchUp))

(event Collision|EventActorBeginOverlap
  (params (OtherActor :type Actor%20Object%20Reference)))

(event Custom|HatchUp
  (Variables|Default|SetOriginHatchRotation (Variables|/Script/Engine.SceneComponent|GetRelativeRotation (Variables|Default|GetSM_Wing_L)))
  (Variables|Default|SetOriginHatchPitch (.pitch (Variables|Default|GetOriginHatchRotation)))
  (bind _alpha (Timeline|TL_HatchUp PlayFromStart)
    (:Update
      (Transformation|SetRelativeRotation (Variables|Default|GetSM_Wing_L) (Math|Rotator|MakeRotator (.roll (Variables|Default|GetOriginHatchRotation)) (Math|Float|Lerp (Variables|Default|GetOriginHatchPitch) (Variables|Default|GetDestHatchPitch) _alpha) (.yaw (Variables|Default|GetOriginHatchRotation))) false false))))

(fn ConstructionScript)